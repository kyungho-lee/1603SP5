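; World map stage button that shows whether its region is cleared, next or locked, and opens that stage's level.
; On BeginPlay, a three-way compare of the game instance's Clearstage against RegionId picks the billboard sprite.
; Clicking an unlocked stage shows a UI_info widget with InfoImage, polls it through a zero-delay loop, then loads TargetLevel on Yes.
; Locked stages show a warning; an older confirm prompt is left unconnected.
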(event `self.ReceiveBeginPlay`
  (bind _billboard (`self.Billboard`))
  (`self.CompBranch` (`/Game/CHS/01BP/BP_Instance.clearstage` (cast `/Game/CHS/01BP/BP_Instance` (`GameplayStatics.GetGameInstance`) :!pure true)) (`self.RegionId`)
    (:`X>Y`
      (`KismetSystemLibrary.PrintString` "완료")
      (`BillboardComponent.SetSprite` _billboard "/Game/sungwon/res/done.done"))
    (:`X=Y`
      (`KismetSystemLibrary.PrintString` "해금")
      (`BillboardComponent.SetSprite` _billboard "/Game/sungwon/res/next.next"))
    (:`X<Y`
      (`KismetSystemLibrary.PrintString` "잠김")
      (`BillboardComponent.SetSprite` _billboard "/Game/sungwon/res/lock.lock"))))

(event `self.click.OnClicked`
  (params (TouchedComponent :type "PrimitiveComponent Object Reference") (ButtonPressed :type "Key Structure"))
  (`self.CompBranch` (`/Game/CHS/01BP/BP_Instance.clearstage` (cast `/Game/CHS/01BP/BP_Instance` (`GameplayStatics.GetGameInstance`) :!pure true)) (`self.RegionId`)
    (:`X>Y`
      (bind _returnvalue (`|CreateWidget` "/Game/sungwon/worldmap/UI_info.UI_info_C" :!label _label))
      (`UserWidget.AddToViewport` _returnvalue 1)
      (`Image.SetBrush` (`/Game/sungwon/worldmap/UI_info.frame` _returnvalue) (make `SlateBrush` (1803.0 1286.0) (struct) (struct :`SpecifiedColor` (struct :`R` 1.0 :`G` 1.0 :`B` 1.0 :`A` 1.0) :`ColorUseRule` "UseColor_Specified") (`self.infoImage`)))
      (if (`/Game/sungwon/worldmap/UI_info.isActive` _returnvalue) :!label _label_2
        (`KismetSystemLibrary.Delay` 0.0) ; 대기하며 루프
        (goto _label_2)
        (elif (`/Game/sungwon/worldmap/UI_info.isYes` _returnvalue)
          (`GameplayStatics.OpenLevel` (`self.targetLevel`)))))
    (:`X=Y`
      (goto _label))
    (:`X<Y`
      (`/Game/sungwon/common/UIConfirmActorBaseMacro.ShowUIConfirm` "잠겼습니다. 이전스테이지를 클리어 해주세요"))))

(fn `UserConstructionScript`)