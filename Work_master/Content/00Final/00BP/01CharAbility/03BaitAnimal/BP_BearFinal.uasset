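; Goal marker for the bait-animal bear feature that detects when a BP_Bait is placed in its FinalLoc zone.
; A timeline bobs the arrow, and the construction script configures the sector particle effect from variables.
; A bait overlap starts a short one-shot timer, then an enlarged sphere trace at the actor rechecks for bait.
; A confirmed hit calls CheckBait on bait and Bear and turns the particles green.
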(event `self.ReceiveBeginPlay`
  (bind (_startloc_x _startloc_y _startloc_z) (`KismetMathLibrary.BreakVector` (`self.StartLoc`)))
  (bind _arrow (`self.Arrow`))
  (set `self.StartLoc` (`SceneComponent.RelativeLocation` _arrow))
  (bind (_direction `_새_트랙_0`) (`Timeline|타임라인_0`)
    (:`Update`
      (`SceneComponent.K2_SetRelativeLocation` _arrow (`KismetMathLibrary.MakeVector` _startloc_x _startloc_y (+ _startloc_z `_새_트랙_0`)) false false))))

(event `CheckStart`
  (`KismetSystemLibrary.K2_SetTimerDelegate` (delegate `BaitTickCheck`) 2.0))

(event `BaitTickCheck`
  (bind _returnvalue (`self.K2_GetActorLocation`))
  (bind (_outhit _returnvalue_2) (`KismetSystemLibrary.SphereTraceSingleForObjects` :`Start` _returnvalue :`End` _returnvalue :`Radius` (* 8 (`SphereComponent.SphereRadius` (`self.FinalLoc`))) :`ObjectTypes` (`|MakeArray` "ObjectTypeQuery10" "ObjectTypeQuery11" :!type "EObjectTypeQuery Enum") :`DrawDebugType` "ForDuration"))
  (if _returnvalue_2
    (bind _asbp_bait (cast `/Game/00Final/00BP/01CharAbility/03BaitAnimal/BP_Bait` (`.HitActor` (`GameplayStatics.BreakHitResult` _outhit))))
    (bind _output_get (set `self.BaitBool` true))
    (`/Game/00Final/00BP/01CharAbility/03BaitAnimal/BP_Bait.CheckBait` _asbp_bait _output_get)
    (`/Game/00Final/00BP/01CharAbility/03BaitAnimal/BP_PolarBear.CheckBait` (`self.Bear`))
    (`FXSystemComponent.SetColorParameter` (`self.ParticleSystem`) "Color" (struct :`R` 0.118336 :`G` 1.0 :`A` 1.0))))

(event `self.FinalLoc.OnComponentBeginOverlap`
  (params (OverlappedComponent :type "PrimitiveComponent Object Reference") (OtherActor :type "Actor Object Reference") (OtherComp :type "PrimitiveComponent Object Reference") (OtherBodyIndex :type Integer) (bFromSweep :type Boolean) (SweepResult :type "HitResult Structure (by ref)"))
  (cast `/Game/00Final/00BP/01CharAbility/03BaitAnimal/BP_Bait` OtherActor)
  (`self.CheckStart`))

(fn `UserConstructionScript`
  (bind _particlesystem (`self.ParticleSystem`))
  (`ParticleSystemComponent.SetTemplate` _particlesystem "/Game/Art/Hemi/ParticleSystem/P_Sector.P_Sector")
  (`PrimitiveComponent.SetMaterial` _particlesystem 0 "/Game/Art/Hemi/ParticleSystem/M_Flare_02_INST.M_Flare_02_INST")
  (`FXSystemComponent.SetColorParameter` _particlesystem "Color" (`self.Color`))
  (`FXSystemComponent.SetFloatParameter` _particlesystem "Spawn" (`self.Spawn`))
  (`FXSystemComponent.SetFloatParameter` _particlesystem "Sphere" (`self.Sphere`)))