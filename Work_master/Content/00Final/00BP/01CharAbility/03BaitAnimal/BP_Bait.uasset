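; BP_Bait is a throwable bait actor that can respawn at its starting spot after being thrown.
; BeginPlay stores the Bait component's location, and Throwed waits a few seconds, then spawns a replacement there and destroys itself if DestroyBool is set.
; CheckBait sets DestroyBool to the inverse of BaitBool.
; Overlap with BP_BearFinal re-enters that same branch, reading BaitBool without passing a new value.
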(event `self.ReceiveBeginPlay`
  (set `self.RespawnLoc` (`SceneComponent.K2_GetComponentLocation` (`self.Bait`))))

(event `CheckBait`
  (params (BaitBool :type Boolean))
  (if BaitBool :!label _label
    (set `self.DestroyBool` false)
    (else
      (set `self.DestroyBool` true))))

(event `self.Bait.OnComponentBeginOverlap`
  (params (OverlappedComponent :type "PrimitiveComponent Object Reference") (OtherActor :type "Actor Object Reference") (OtherComp :type "PrimitiveComponent Object Reference") (OtherBodyIndex :type Integer) (bFromSweep :type Boolean) (SweepResult :type "HitResult Structure (by ref)"))
  (cast `/Game/00Final/00BP/01CharAbility/03BaitAnimal/BP_BearFinal` OtherActor)
  (goto _label))

(event `Throwed`
  (`KismetSystemLibrary.Delay` 5.0)
  (if (`self.DestroyBool`)
    (`|SpawnActorFromClass` "BP_Bait_C" (`KismetMathLibrary.MakeTransform` (`self.RespawnLoc`)) "Undefined" "OverrideRootScale" null null)
    (`/Engine/EditorBlueprintResources/StandardMacros.IsValid` self
      (:`Is Valid`
        (`self.K2_DestroyActor`)))))

(fn `UserConstructionScript`)