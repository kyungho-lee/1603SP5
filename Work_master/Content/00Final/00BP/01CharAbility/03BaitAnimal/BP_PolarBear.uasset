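; Polar bear bait-animal character that walks toward set goals and turns follower actors it touches into meat.
; StartBear runs a looping timer that moves it to FirstLoc, or to FinalLoc once CheckBait flips the goal.
; Before that switch, a Bee flag halts it until a long delay clears the flag.
; Overlapping a JustFollow dissolves and destroys it, spawns BP_Meat with a cook message, and plays the bear montage once.
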(event `/Game/00Final/00BP/01CharAbility/03BaitAnimal/BPI_CheckBait.StartBear`
  (bind _returnvalue (`KismetSystemLibrary.K2_SetTimerDelegate` (delegate `MoveToLocationEvent`) 0.2 true))
  (set `self.MoveHandler` _returnvalue))

(event `MoveToLocationEvent`
  (bind _returnvalue (`self.GetController` self))
  (set `CharacterMovementComponent.MaxWalkSpeed` (`self.WalkSpeed`) (`self.CharacterMovement`))
  (if (`self.ChangeGoal`)
    (`AIBlueprintHelperLibrary.SimpleMoveToActor` _returnvalue (`self.FinalLoc`))
    (elif (`self.Bee`)
      (`Controller.StopMovement` _returnvalue)
      (`KismetSystemLibrary.Delay` 50.0)
      (set `self.Bee` false)
      (else
        (`AIBlueprintHelperLibrary.SimpleMoveToActor` _returnvalue (`self.FirstLoc`))))))

(event `/Game/00Final/00BP/01CharAbility/03BaitAnimal/BPI_CheckBait.CheckBait`
  (set `self.ChangeGoal` true))

(event `self.DestroyFollower.OnComponentBeginOverlap`
  (params (OverlappedComponent :type "PrimitiveComponent Object Reference") (OtherActor :type "Actor Object Reference") (OtherComp :type "PrimitiveComponent Object Reference") (OtherBodyIndex :type Integer) (bFromSweep :type Boolean) (SweepResult :type "HitResult Structure (by ref)"))
  (bind _asjust_follow (cast `/Game/00Final/00BP/00BaseSystem/JustFollow` OtherActor))
  (`|ExecutionSequence`
    (:`then_0`
      (`/Game/00Final/00BP/00BaseSystem/JustFollow.DissolveEffect` _asjust_follow))
    (:`then_1`
      (bind _returnvalue (`|SpawnActorFromClass` "/Game/Art/Hemi/BluePrints/BP_Meat.BP_Meat_C" (`KismetMathLibrary.Conv_VectorToTransform` (`.ImpactPoint` (`GameplayStatics.BreakHitResult` SweepResult))) "Undefined" "OverrideRootScale" null null))
      (message `/Game/Art/Hemi/BluePrints/BPI_Cook.Cook` _returnvalue)
      (`KismetSystemLibrary.Delay` 1.0)
      (`/Engine/EditorBlueprintResources/StandardMacros.IsValid` _asjust_follow
        (:`Is Valid`
          (`self.K2_DestroyActor` _asjust_follow))))
    (:`then_2`
      (`/Engine/EditorBlueprintResources/StandardMacros.DoOnce` false
        (:`Completed`
          (`self.PlayAnimMontage` "/Game/Art/Hemi/Bear/ANIMMON_Enemy_Bear.ANIMMON_Enemy_Bear"))))))

(event `self.ReceiveBeginPlay`)

(fn `UserConstructionScript`)