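; BP_PullActor, filed under the Rope character ability, is a spawner that drops a batch of physics-driven BP_FillObject actors around itself.
; On BeginPlay, a fast looping timer counts SpawnNum down and spawns one object per tick at a random point in a flat box.
; Each object is stretched, its mesh rotated, and collision and physics simulation enabled.
; The timer handle is stored but never cleared, so it keeps firing after the count runs out.
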(event `self.ReceiveBeginPlay`
  (bind _returnvalue (`KismetSystemLibrary.K2_SetTimerDelegate` (delegate `SpawnPullActor`) 0.05 true))
  (set `self.SpawnHandler` _returnvalue))

(event `SpawnPullActor`
  (bind _spawnnum (`self.SpawnNum`))
  (`/Engine/EditorBlueprintResources/StandardMacros.DecrementInt` _spawnnum
    (:`  `
      (if (>= _spawnnum 0)
        (bind _returnvalue (`|SpawnActorFromClass` "/Game/00Final/00BP/01CharAbility/02FillHole/BP_FillObject.BP_FillObject_C" (`KismetMathLibrary.Conv_VectorToTransform` (`KismetMathLibrary.RandomPointInBoundingBox` (`self.K2_GetActorLocation`) (100.0 150.0 1.0))) "AdjustIfPossibleButAlwaysSpawn" "OverrideRootScale" null null))
        (`/Engine/EditorBlueprintResources/StandardMacros.IsValid` _returnvalue
          (:`Is Valid`
            (`self.SetActorRelativeScale3D` _returnvalue (1.0 1.0 5.0))
            (bind _staticmeshcomponent (`StaticMeshActor.StaticMeshComponent` _returnvalue))
            (`SceneComponent.K2_AddWorldRotation` _staticmeshcomponent (struct :`Yaw` -15.0 :`Roll` 90.0) false false)
            (`PrimitiveComponent.SetCollisionEnabled` _staticmeshcomponent "QueryAndPhysics")
            (`PrimitiveComponent.SetSimulatePhysics` _staticmeshcomponent true)))))))

(fn `UserConstructionScript`)