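; BP_Leader is an invisible-or-visible guide actor that leads spawned JustFollow characters along a patrol spline.
; On BeginPlay it spawns CharSpawn followers nearby, setting their mesh, animation, speed, controller and follow target.
; A looping timer sphere-traces for a follower and, only when one is within range, advances the leader by PatrolSpeed along FollowingPath's spline.
; Distance resets when the path changes, and movement stops at the spline's end.
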(event `self.ReceiveBeginPlay`
  (set `self.BeforePath` (`self.FollowingPath`))
  (while (> (`self.CharSpawn`) 0)
    ;[0.5851 1 0.4775] 팔로잉 오브젝트 스폰(설정 갯수만큼)
    (bind _returnvalue (`|SpawnActorFromClass` "/Game/00Final/00BP/00BaseSystem/JustFollow.JustFollow_C" (`KismetMathLibrary.Conv_VectorToTransform` (`KismetMathLibrary.RandomPointInBoundingBox` (+ (`self.K2_GetActorLocation`) (0.0 0.0 60.0)) (300.0 300.0 50.0))) "AdjustIfPossibleButAlwaysSpawn" "OverrideRootScale" null null))
    (`SkinnedMeshComponent.SetSkinnedAssetAndUpdate` (`Character.Mesh` _returnvalue) (`self.SpawnMesh`) true)
    (set `/Game/00Final/00BP/00BaseSystem/JustFollow.FollowerSpeed` (`self.FollowerSpeed`) _returnvalue)
    (`SkeletalMeshComponent.SetAnimInstanceClass` (`Character.Mesh` _returnvalue) (`self.SpawnAnimClass`))
    (`Pawn.SpawnDefaultController` _returnvalue)
    (set `/Game/00Final/00BP/00BaseSystem/JustFollow.FollowActor` self _returnvalue)
    (set `self.Follower` _returnvalue)
    (`/Engine/EditorBlueprintResources/StandardMacros.DecrementInt` (`self.CharSpawn`)
      (:`  `
        (if (`KismetSystemLibrary.IsValid` _returnvalue)
          (`/Engine/EditorBlueprintResources/StandardMacros.IncrementInt` (`self.CheckSpawn`))))))
  (`KismetSystemLibrary.PrintString` (`KismetStringLibrary.Conv_IntToString` (`self.CheckSpawn`)))
  ;[0.2702 1 0.75] Leader Actor Move
  (bind _returnvalue_2 (`KismetSystemLibrary.K2_SetTimerDelegate` (delegate `Patrol`) 0.3 true))
  (set `self.PatrolHandle` _returnvalue_2))

(event `Patrol`
  (bind _returnvalue (`self.K2_GetActorLocation`))
  ;[0.2702 1 0.75] Leader Actor Move
  (if (!= (`self.FollowingPath`) (`self.BeforePath`))
    (set `self.BeforePath` (`self.FollowingPath`))
    (set `self.Distance` 0.0))
  (bind _outhit (`KismetSystemLibrary.SphereTraceSingleForObjects` _returnvalue _returnvalue 300.0 (`|MakeArray` "ObjectTypeQuery13" :!type "EObjectTypeQuery Enum")))
  (bind _asjust_follow (cast `/Game/00Final/00BP/00BaseSystem/JustFollow` (`.HitActor` (`GameplayStatics.BreakHitResult` _outhit))))
  (set `self.Follower` _asjust_follow)
  (if (<= (`KismetMathLibrary.VSizeXY` (- (`self.K2_GetActorLocation` (`self.Follower`)) (`self.K2_GetActorLocation`))) 300.0)
    (bind _output_get (set `self.Distance` (+ (`self.Distance`) (`self.PatrolSpeed`))))
    ;;[0.8323 0.4077 1] False일 경우 해당 Spline의 끝지점 도달
    (if (< _output_get (`SplineComponent.GetSplineLength` (`/Game/00Final/00BP/00BaseSystem/BP_SimplePath.PatrolSpline` (`self.FollowingPath`))))
      (bind _output_get_2 (set `self.TargetLocation` (`SplineComponent.GetLocationAtDistanceAlongSpline` (`/Game/00Final/00BP/00BaseSystem/BP_SimplePath.PatrolSpline` (`self.FollowingPath`)) (`self.Distance`) "World")))
      (`self.K2_SetActorLocation` _output_get_2))))

(fn `UserConstructionScript`)