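; BP_BubbleEmitter spawns BP_Bubble actors at random level TargetPoints, playing a bubbling sound each time.
; BubbleEmit spawns only while the count is at or below BubbleLimit, behind an IsSpawing flag that clears immediately afterwards.
; Each spawn increments HowManyBubbles, prints it and passes it on through CallHowManyHaveYougot.
; The random index range includes the array length, so it can land out of bounds.
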(event `/Game/00Final/02ArtBP/BluePrints/BPI_BubbleEmit.BubbleEmit`
  (if (and (<= (`self.HowManyBubbles`) (`self.BubbleLimit`)) (!= (`self.IsSpawing?`) true))
    (bind _outactors (`GameplayStatics.GetAllActorsOfClass` "/Script/Engine.TargetPoint"))
    (`|SpawnActorFromClass` "/Game/00Final/02ArtBP/BluePrints/BP_Bubble.BP_Bubble_C" (`self.GetTransform` (`|GetArrayItem` _outactors (`KismetMathLibrary.RandomIntegerInRange` 0 (`KismetArrayLibrary.Array_Length` _outactors)))) "AlwaysSpawn" "OverrideRootScale" null null)
    (`GameplayStatics.PlaySound2D` "/Game/Art/Hemi/Sounds/BubblingSound.BubblingSound" 1.0 1.0 0.0 null null)
    (set `self.IsSpawing?` true)
    (`|ExecutionSequence`
      (:`then_0`
        (set `self.IsSpawing?` false))
      (:`then_1`
        (bind _output_get (set `self.Bubble` 1))
        (bind _output_get_2 (set `self.HowManyBubbles` (+ (`self.HowManyBubbles`) _output_get)))
        (`KismetSystemLibrary.PrintString` (`KismetStringLibrary.Conv_IntToString` _output_get_2))
        (`self.HowManyHaveYougot` _output_get_2)))))

(fn `UserConstructionScript`)