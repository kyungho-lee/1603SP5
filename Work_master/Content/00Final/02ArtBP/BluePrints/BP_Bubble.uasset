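; BP_Bubble is a bubble actor that can float along a path and pops once a count reported by BP_BubbleEmitter exceeds its limit.
; Overlapping a BP_RasieUP with its sphere plays a timeline that lerps the bubble mesh from Start to End.
; It binds to the emitter's HowManyHaveYougot dispatcher; on popping it plays a sound, destroys itself, sends BoomMessage to BP_RainbowBridge and destroys the emitter.
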(event `self.Sphere.OnComponentBeginOverlap`
  (params (OverlappedComponent :type "PrimitiveComponent Object Reference") (OtherActor :type "Actor Object Reference") (OtherComp :type "PrimitiveComponent Object Reference") (OtherBodyIndex :type Integer) (bFromSweep :type Boolean) (SweepResult :type "HitResult Structure (by ref)"))
  (cast `/Game/00Final/02ArtBP/BluePrints/BP_RasieUP` OtherActor)
  (bind (_direction _newtrack_0) (`Timeline|Timeline_0`)
    (:`Update`
      (`SceneComponent.K2_SetRelativeLocation` (`self.Bubble`) (`KismetMathLibrary.VLerp` (`self.start`) (`self.end`) _newtrack_0) false false))))

(event `self.ReceiveBeginPlay`
  (bind _returnvalue (`GameplayStatics.GetActorOfClass` "/Game/00Final/02ArtBP/BluePrints/BP_BubbleEmitter.BP_BubbleEmitter_C"))
  (add `/Game/00Final/02ArtBP/BluePrints/BP_BubbleEmitter.HowManyHaveYougot` _returnvalue (delegate `HowManyHaveYougot_Event_0`)))

(event `HowManyHaveYougot_Event_0`
  (params (HowMany :type Integer))
  (`KismetSystemLibrary.PrintString` "I'mHearing")
  (if (> HowMany (`self.Limit`))
    (`GameplayStatics.PlaySound2D` "/Game/Art/Hemi/Sounds/BubblePop.BubblePop" 0.1 1.0 0.0 null null)
    (`self.K2_DestroyActor`)
    (`|ExecutionSequence`
      (:`then_0`
        (`KismetSystemLibrary.PrintString` "Boom")
        (bind _returnvalue (`GameplayStatics.GetActorOfClass` "/Game/00Final/02ArtBP/BluePrints/BP_RainbowBridge.BP_RainbowBridge_C"))
        (message `/Game/00Final/02ArtBP/BluePrints/BPI_Boom.Boom` _returnvalue))
      (:`then_1`
        (bind _returnvalue_2 (`GameplayStatics.GetActorOfClass` "/Game/00Final/02ArtBP/BluePrints/BP_BubbleEmitter.BP_BubbleEmitter_C"))
        (`self.K2_DestroyActor` _returnvalue_2)))))

(fn `UserConstructionScript`)