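; BP_FireWorks is a firework effect Blueprint that shows a particle system with constantly changing random colors.
; StartFireWork sets a running flag and makes the particle system visible.
; While the flag is set, Tick calls ChangeColor, which creates a new dynamic instance of M_FireworksDot1 on material element 2 every frame and sets its Color parameter from a random unit vector.
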(event `StartFireWork`
  (set `self.FireWorkRun` true)
  (`SceneComponent.SetVisibility` (`self.ParticleSystem`) true false))

(event `self.ReceiveTick`
  (params (DeltaSeconds :type "Float (single-precision)"))
  (if (`self.FireWorkRun`)
    (`self.ChangeColor`)))

(event `ChangeColor`
  (bind _returnvalue (`PrimitiveComponent.CreateDynamicMaterialInstance` (`self.ParticleSystem`) 2 "/Game/Art/Hemi/ParticleSystem/M_FireworksDot1.M_FireworksDot1" "None"))
  (`MaterialInstanceDynamic.SetVectorParameterValue` _returnvalue "Color" (`KismetMathLibrary.Conv_VectorToLinearColor` (`KismetMathLibrary.RandomUnitVector`))))

(fn `UserConstructionScript`)