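; Level design tool actor that scatters random static meshes around itself.
; Its construction script adds NumberOfMeshes components, each with a mesh picked at random from MeshesToSpawn.
; Each gets a random XY offset length-clamped to Radius for a circular area, optional random yaw, and per-axis random scale between minimum and maximum.
; The mesh-count clamp is not in effect, so the loop uses the raw value.
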(fn `UserConstructionScript`
  (bind _radius (`self.Radius`))
  (bind _meshes_to_spawn (`self.Meshes to spawn`))
  (bind _returnvalue (* _radius -1.0))
  (set `self.Count` (- (`KismetMathLibrary.Clamp` (`self.Number of meshes`) 1 20) 1))
  (for _ (range 1 (+ (`self.Number of meshes`) 1))
    (bind _returnvalue_2 (`AddComponent|NODE_AddStaticMeshComponent-0` :`RelativeTransform` (`KismetMathLibrary.MakeTransform` (`KismetMathLibrary.ClampVectorSize` (`KismetMathLibrary.MakeVector` (`KismetMathLibrary.RandomFloatInRange` _returnvalue _radius) (`KismetMathLibrary.RandomFloatInRange` _returnvalue _radius)) 0.0 (`self.Radius`)) (`KismetMathLibrary.SelectRotator` (`KismetMathLibrary.MakeRotator` 0.0 0.0 (`KismetMathLibrary.RandomFloatInRange` 0.0 360.0)) (struct) (`self.Random yaw rotation`)) (`KismetMathLibrary.MakeVector` (`KismetMathLibrary.RandomFloatInRange` (.x (`self.Minimum scale`)) (.x (`self.Maximum scale`))) (`KismetMathLibrary.RandomFloatInRange` (.y (`self.Minimum scale`)) (.y (`self.Maximum scale`))) (`KismetMathLibrary.RandomFloatInRange` (.z (`self.Minimum scale`)) (.z (`self.Maximum scale`)))))))
    (`StaticMeshComponent.SetStaticMesh` _returnvalue_2 (`|GetArrayItem` _meshes_to_spawn (`KismetMathLibrary.RandomIntegerInRange` 0 (`KismetArrayLibrary.Array_LastIndex` _meshes_to_spawn)))) ; Change the new static mesh to the specified type
  ))