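; BP_PlaceInLine is a level design tool actor that places copies of a chosen static mesh in a straight line.
; Its Construction Script adds one mesh component per Count, clamped between 1 and 20, all sharing a configurable yaw.
; Each copy is offset from the previous one along local negative Y by a scaled Distance, accumulated in NewMeshLocation.
; The event graph has no logic.
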(fn `UserConstructionScript`
  (for _ (range (`KismetMathLibrary.Clamp` (`self.Count`) 1 20))
    (bind _returnvalue (`AddComponent|NODE_AddStaticMeshComponent-0` :`RelativeTransform` (`KismetMathLibrary.MakeTransform` (`self.NewMeshLocation`) (`KismetMathLibrary.MakeRotator` 0.0 0.0 (`self.Rotate Y`)))))
    (`StaticMeshComponent.SetStaticMesh` _returnvalue (`self.StaticMesh`))
    (set `self.NewMeshLocation` (+ (`self.NewMeshLocation`) (`KismetMathLibrary.MakeVector` 0.0 (* (`self.Distance`) -50.0))))))