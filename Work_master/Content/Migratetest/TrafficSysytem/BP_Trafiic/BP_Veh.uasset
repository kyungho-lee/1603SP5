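; BP_Veh is a traffic vehicle that moves along the spline of a referenced track and halts on red signals.
; If active, it starts the CartMover timeline on BeginPlay, with play rate from Duration and start time from VehStartOffset.
; The timeline's Alpha maps to distance along the spline, setting the actor's location and rotation each update.
; The traffic controller interface event passes IsRed to stop or resume the timeline.
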(event `self.ReceiveBeginPlay`
  ;[1 1 1] Move Car
  (if (`self.activeVeh`)
    (`self.MoveCart`)))

(event `MoveCart`
  (bind _returnvalue (`KismetMathLibrary.Lerp` 0.0 (`SplineComponent.GetSplineLength` (`/Game/Migratetest/TrafficSysytem/BP_Trafiic/BP_Track.UsefulSpline` (`self.TrackRef`))) (`self.Alpha`)))
  ;[1 1 1] Controll the speed and offset, moving of the car
  (`TimelineComponent.SetPlayRate` (`self.CartMover`) (/ 1.0 (`self.Duration`)))
  (`TimelineComponent.SetNewTime` (`self.CartMover`) (`self.VehStartOffset`))
  (if (stale `/Game/Migratetest/TrafficSysytem/BP_Trafiic/BPI_CentreControll.BPI_TrafficContoller` `isRed?`) :!label _label
    (`KismetSystemLibrary.PrintString` "Stop")
    (bind (_direction _alpha) (`Timeline|CartMover` :!via `Stop` :!label _label_2)
      (:`Update`
        (set `self.Alpha` _alpha)
        (`self.K2_SetActorLocationAndRotation` (`SplineComponent.GetLocationAtDistanceAlongSpline` (`/Game/Migratetest/TrafficSysytem/BP_Trafiic/BP_Track.UsefulSpline` (`self.TrackRef`)) _returnvalue "World") (`SplineComponent.GetRotationAtDistanceAlongSpline` (`/Game/Migratetest/TrafficSysytem/BP_Trafiic/BP_Track.UsefulSpline` (`self.TrackRef`)) _returnvalue "World"))))
    (else
      (`KismetSystemLibrary.PrintString` "Go")
      (goto _label_2))))

(event `/Game/Migratetest/TrafficSysytem/BP_Trafiic/BPI_CentreControll.BPI_TrafficContoller`
  (params (`isRed?` :type Boolean))
  ;[1 1 1] Controll the speed and offset, moving of the car
  (goto _label))

(fn `UserConstructionScript`)