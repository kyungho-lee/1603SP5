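; BP_TrafficSign is a traffic light that turns red while a ThirdPersonCharacter overlaps it and green when the overlap ends.
; Construction starts it green by hiding the Red and Yellow components.
; Each change sets IsRed and toggles Green and Red visibility rather than setting it explicitly.
; It then broadcasts IsRed through BPITrafficContollerMessage to every actor implementing BPI_CentreControll, found by a world-wide interface search.
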(event `self.ReceiveActorBeginOverlap`
  (params (OtherActor :type "Actor Object Reference"))
  ;[1 1 1] Trigger Red And Green light
  (cast `/Game/Migratetest/ThirdPersonCharacter` OtherActor)
  (`self.Red Light`))

(event `self.ReceiveActorEndOverlap`
  (params (OtherActor :type "Actor Object Reference"))
  ;[1 1 1] Trigger Red And Green light
  (cast `/Game/Migratetest/ThirdPersonCharacter` OtherActor)
  (`self.Green light`))

(event `Green light`
  ;[1 1 1] Green Light
  (bind _output_get (set `self.isRed?` false))
  (if (not _output_get)
    (`KismetSystemLibrary.Delay` 0.0)
    (`SceneComponent.ToggleVisibility` (`self.Green`) false)
    (`SceneComponent.ToggleVisibility` (`self.Red`) false)
    (`|ExecutionSequence`
      (:`then_0`
        (bind _outactors (`GameplayStatics.GetAllActorsWithInterface` "/Game/Migratetest/TrafficSysytem/BP_Trafiic/BPI_CentreControll.BPI_CentreControll_C"))
        (for _array_element _outactors
          (message `/Game/Migratetest/TrafficSysytem/BP_Trafiic/BPI_CentreControll.BPI_TrafficContoller` _array_element (stale _output_get_2) :!label _label)
          (`KismetSystemLibrary.PrintString` "Greenlight")))
      (:`then_1`
        (bind _output_get_2 (set `self.isRed?` false))
        (goto _label)))))

(event `Red Light`
  ;[1 1 1] Red Light
  (bind _output_get (set `self.isRed?` true))
  (if _output_get
    (`KismetSystemLibrary.Delay` 0.0)
    (`SceneComponent.ToggleVisibility` (`self.Green`) false)
    (`SceneComponent.ToggleVisibility` (`self.Red`) false)
    (`|ExecutionSequence`
      (:`then_0`
        (bind _outactors (`GameplayStatics.GetAllActorsWithInterface` "/Game/Migratetest/TrafficSysytem/BP_Trafiic/BPI_CentreControll.BPI_CentreControll_C"))
        (for _array_element _outactors
          (message `/Game/Migratetest/TrafficSysytem/BP_Trafiic/BPI_CentreControll.BPI_TrafficContoller` _array_element (stale _output_get_2) :!label _label_2)))
      (:`then_1`
        (bind _output_get_2 (set `self.isRed?` true))
        (goto _label_2)))))

(fn `UserConstructionScript`
  (bind _output_get (set `self.isRed?` false))
  (if (not _output_get)
    (`SceneComponent.SetVisibility` (`self.Red`) false false)
    (`SceneComponent.SetVisibility` (`self.Yellow`) false false)))