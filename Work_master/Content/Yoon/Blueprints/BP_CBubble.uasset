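; BP_CBubble is a character-style Blueprint with a timed bubble state that makes it fly.
; VisibleBubble shows the mesh, simulates physics on the capsule without gravity, then calls InvisibleBubble after a delay.
; While flying, Tick pushes the capsule upward from an offset above its origin or along Dir, depending on the Up flag.
; InvisibleBubble hides the mesh, restores gravity, resets rotation and stops physics simulation.
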(event `VisibleBubble`
  (`SceneComponent.K2_SetRelativeRotation` :`self` (`self.CapsuleComponent`))
  (`PrimitiveComponent.SetSimulatePhysics` (`self.CapsuleComponent`) false)
  (`PrimitiveComponent.SetSimulatePhysics` (`self.CapsuleComponent`) true)
  (`PrimitiveComponent.SetEnableGravity` (`self.CapsuleComponent`) false)
  (`SceneComponent.SetVisibility` (`self.StaticMesh`) true false)
  (set `self.CanFly` true)
  (`KismetSystemLibrary.Delay` (`self.BubbleDelay`))
  (`self.InvisibleBubble`))

(event `self.ReceiveTick`
  (params (DeltaSeconds :type "Float (single-precision)"))
  (if (`self.CanFly`)
    (if (`self.Up`)
      (`PrimitiveComponent.AddForceAtLocation` (`self.CapsuleComponent`) (* (0.0 0.0 1.0) (`self.Force`)) (+ (`SceneComponent.K2_GetComponentLocation` (`self.CapsuleComponent`)) (0.0 0.0 50.0)) "None")
      (else
        (`PrimitiveComponent.AddForceAtLocation` (`self.CapsuleComponent`) (* (`self.Dir`) (`self.Force`)) (+ (`SceneComponent.K2_GetComponentLocation` (`self.CapsuleComponent`)) (0.0 0.0 0.0)) "None")))))

(event `InvisibleBubble`
  (`PrimitiveComponent.SetEnableGravity` (`self.CapsuleComponent`) true)
  (`SceneComponent.SetVisibility` (`self.StaticMesh`) false false)
  (set `self.CanFly` false)
  (`SceneComponent.K2_SetRelativeRotation` :`self` (`self.CapsuleComponent`))
  (`PrimitiveComponent.SetSimulatePhysics` (`self.CapsuleComponent`) false))

(fn `UserConstructionScript`)