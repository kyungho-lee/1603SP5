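; Floating skeletal-mesh actor, apparently a penguin judging by its dissolve material, that removes itself shortly after spawning.
; Tick passes the mesh, a buoyancy start value and a collision channel to BuoyancyFunction to keep it afloat.
; A one-shot timer from BeginPlay swaps in a dynamic dissolve material and plays a timeline that sets its Dissolve parameter, then destroys the actor when finished.
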(event `self.ReceiveBeginPlay`
  (`KismetSystemLibrary.K2_SetTimerDelegate` (delegate `DissolveEffect`) 5.0))

(event `DissolveEffect`
  (bind _skeletalmesh (`self.SkeletalMesh`))
  ;[1 1 1] 사라지는 효과
  (`PrimitiveComponent.SetMaterial` _skeletalmesh 0 "/Game/Art/Hemi/Materials/MI_DissolvePenguin.MI_DissolvePenguin")
  (bind _returnvalue (`PrimitiveComponent.CreateDynamicMaterialInstance` _skeletalmesh 0 "/Game/Art/Hemi/Materials/MI_DissolvePenguin.MI_DissolvePenguin" "None"))
  (`Timeline|타임라인_0`
    (:`Update`
      (`MaterialInstanceDynamic.SetScalarParameterValue` _returnvalue "Dissolve" 0.0))
    (:`Finished`
      (`self.K2_DestroyActor`))))

(event `self.ReceiveTick`
  (params (DeltaSeconds :type "Float (single-precision)"))
  (`/Game/Yoon/Blueprints/BuoyancyFuntion.Buoyancy Function` (`self.SkeletalMesh`) (`self.BuoyancyStart`) "ObjectTypeQuery7"))

(fn `UserConstructionScript`)