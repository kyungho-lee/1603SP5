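; BP_BB is an actor that reacts to a BP_ actor hitting it by exploding and swapping to a second mesh.
; When the StaticMesh component begins overlapping a BP_, it destroys that actor and spawns the P_Explosion emitter at the mesh's location.
; It then hides the StaticMesh and disables its collision, while showing the Cube and enabling its query and physics collision.
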(event `self.StaticMesh.OnComponentBeginOverlap`
  (params (OverlappedComponent :type "PrimitiveComponent Object Reference") (OtherActor :type "Actor Object Reference") (OtherComp :type "PrimitiveComponent Object Reference") (OtherBodyIndex :type Integer) (bFromSweep :type Boolean) (SweepResult :type "HitResult Structure (by ref)"))
  (bind _staticmesh (`self.StaticMesh`))
  (bind _asbp_ (cast `/Game/Yoon/Blueprints/BP_` OtherActor))
  (`self.K2_DestroyActor` _asbp_)
  (`GameplayStatics.SpawnEmitterAtLocation` "/Game/UnrealDefaultAsset/StarterContent/Particles/P_Explosion.P_Explosion" (`SceneComponent.K2_GetComponentLocation` (`self.StaticMesh`)))
  (`SceneComponent.SetVisibility` (`self.Cube`) true false)
  (`SceneComponent.SetVisibility` _staticmesh false false)
  (`PrimitiveComponent.SetCollisionEnabled` _staticmesh "NoCollision")
  (`PrimitiveComponent.SetCollisionEnabled` (`self.Cube`) "QueryAndPhysics"))

(fn `UserConstructionScript`)