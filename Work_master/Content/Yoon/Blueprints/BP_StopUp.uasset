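; BP_StopUp is a trigger actor that steers and removes JustFollow actors as they pass through its volumes.
; UpBox sets their Up flag on entry, then on exit clears it and sets their Dir to the Arrow component's forward vector.
; StopBox sets Up and calls InvisibleBubble on them, while the Death volume destroys them.
; Each overlap handler casts to JustFollow and ignores anything else.
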(event `self.UpBox.OnComponentBeginOverlap`
  (params (OverlappedComponent :type "PrimitiveComponent Object Reference") (OtherActor :type "Actor Object Reference") (OtherComp :type "PrimitiveComponent Object Reference") (OtherBodyIndex :type Integer) (bFromSweep :type Boolean) (SweepResult :type "HitResult Structure (by ref)"))
  (bind _asjust_follow (cast `/Game/CHS/02FollowPathUnit/01SimplePathMover/JustFollow` OtherActor))
  (set `/Game/CHS/02FollowPathUnit/01SimplePathMover/JustFollow.Up` true _asjust_follow))

(event `self.UpBox.OnComponentEndOverlap`
  (params (OverlappedComponent :type "PrimitiveComponent Object Reference") (OtherActor :type "Actor Object Reference") (OtherComp :type "PrimitiveComponent Object Reference") (OtherBodyIndex :type Integer))
  (bind _asjust_follow (cast `/Game/CHS/02FollowPathUnit/01SimplePathMover/JustFollow` OtherActor))
  (set `/Game/CHS/02FollowPathUnit/01SimplePathMover/JustFollow.Dir` (`SceneComponent.GetForwardVector` (`self.Arrow`)) _asjust_follow)
  (set `/Game/CHS/02FollowPathUnit/01SimplePathMover/JustFollow.Up` false _asjust_follow))

(event `self.StopBox.OnComponentBeginOverlap`
  (params (OverlappedComponent :type "PrimitiveComponent Object Reference") (OtherActor :type "Actor Object Reference") (OtherComp :type "PrimitiveComponent Object Reference") (OtherBodyIndex :type Integer) (bFromSweep :type Boolean) (SweepResult :type "HitResult Structure (by ref)"))
  (bind _asjust_follow (cast `/Game/CHS/02FollowPathUnit/01SimplePathMover/JustFollow` OtherActor))
  (set `/Game/CHS/02FollowPathUnit/01SimplePathMover/JustFollow.Up` true _asjust_follow)
  (`/Game/CHS/02FollowPathUnit/01SimplePathMover/JustFollow.InvisibleBubble` _asjust_follow))

(event `self.Death.OnComponentBeginOverlap`
  (params (OverlappedComponent :type "PrimitiveComponent Object Reference") (OtherActor :type "Actor Object Reference") (OtherComp :type "PrimitiveComponent Object Reference") (OtherBodyIndex :type Integer) (bFromSweep :type Boolean) (SweepResult :type "HitResult Structure (by ref)"))
  (bind _asjust_follow (cast `/Game/CHS/02FollowPathUnit/01SimplePathMover/JustFollow` OtherActor))
  (`self.K2_DestroyActor` _asjust_follow))

(fn `UserConstructionScript`)