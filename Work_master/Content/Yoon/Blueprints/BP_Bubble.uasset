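; BP_Bubble is an actor that lifts a physics mesh inside a visible bubble for a few seconds, then drops it.
; VisibleBubble resets the mesh's rotation and physics, disables gravity, shows the bubble and enables flight, during which Tick applies a scaled forward-and-up force at the mesh's location.
; After a fixed delay, InvisibleBubble restores gravity, hides the bubble, stops flight and resets rotation and physics again.
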(event `self.ReceiveBeginPlay`)

(event `self.ReceiveTick`
  (params (DeltaSeconds :type "Float (single-precision)"))
  (if (`self.CanFly`)
    (`PrimitiveComponent.AddForceAtLocation` (`self.Mesh2`) (* (1.0 0.0 2.0) (`self.Force`)) (+ (`SceneComponent.K2_GetComponentLocation` (`self.Mesh2`)) (0.0 0.0 0.0)) "None")))

(event `VisibleBubble`
  (`SceneComponent.K2_SetRelativeRotation` :`self` (`self.Mesh2`))
  (`PrimitiveComponent.SetSimulatePhysics` (`self.Mesh2`) false)
  (`PrimitiveComponent.SetSimulatePhysics` (`self.Mesh2`) true)
  (`PrimitiveComponent.SetEnableGravity` (`self.Mesh2`) false)
  (`SceneComponent.SetVisibility` (`self.Bubble1`) true false)
  (set `self.CanFly` true)
  (`KismetSystemLibrary.Delay` 4.0)
  (`self.InvisibleBubble`))

(event `InvisibleBubble`
  (`PrimitiveComponent.SetEnableGravity` (`self.Mesh2`) true)
  (`SceneComponent.SetVisibility` (`self.Bubble1`) false false)
  (set `self.CanFly` false)
  (`SceneComponent.K2_SetRelativeRotation` :`self` (`self.Mesh2`))
  (`PrimitiveComponent.SetSimulatePhysics` (`self.Mesh2`) false)
  (`PrimitiveComponent.SetSimulatePhysics` (`self.Mesh2`) true))

(fn `UserConstructionScript`)