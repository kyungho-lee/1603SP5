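; BP_Balloon is a physics balloon that can be tied to another component and lifts it.
; Each tick an upward force is applied above the balloon's origin, and construction gives it a random color through a dynamic material.
; AttachEvent links balloon and target with a physics constraint and pins the cable end at the hit point in the target's local space.
; A lifespan timer destroys it, spawning an explosion emitter.
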(event `self.ReceiveBeginPlay`
  (`self.SetLifeSpan` (`self.LifeTime`)))

(event `self.ReceiveTick`
  (params (DeltaSeconds :type "Float (single-precision)"))
  (`PrimitiveComponent.AddForceAtLocation` (`self.Balloon`) (* (0.0 0.0 1.0) (`self.Force`)) (+ (`SceneComponent.K2_GetComponentLocation` (`self.Balloon`)) (0.0 0.0 100.0)) "None"))

(event `AttachEvent`
  (params (AttachComponent :type "PrimitiveComponent Object Reference") (AttachLocation :type "Vector Structure") (AttachBornName :type Name))
  (bind _cable (`self.Cable`))
  (`PhysicsConstraintComponent.SetConstrainedComponents` (`self.PhysicsConstraint`) AttachComponent AttachBornName (`self.Balloon`) "None")
  (`CableComponent.SetAttachEndToComponent` _cable AttachComponent "None")
  (set `CableComponent.EndLocation` (`KismetMathLibrary.InverseTransformLocation` (`SceneComponent.K2_GetComponentToWorld` AttachComponent) AttachLocation) _cable))

(event `self.ReceiveDestroyed`
  (`GameplayStatics.SpawnEmitterAtLocation` "/Game/UnrealDefaultAsset/StarterContent/Particles/P_Explosion.P_Explosion" (`SceneComponent.K2_GetComponentLocation` (`self.Balloon`))))

(fn `UserConstructionScript`
  (bind _returnvalue (`PrimitiveComponent.CreateDynamicMaterialInstance` (`self.Balloon`) 0 null "BalloonColor"))
  (`MaterialInstanceDynamic.SetVectorParameterValue` _returnvalue "Color" (`KismetMathLibrary.MakeColor` (`KismetMathLibrary.RandomFloatInRange` 0.0 1.0) (`KismetMathLibrary.RandomFloatInRange` 0.0 1.0) (`KismetMathLibrary.RandomFloatInRange` 0.0 1.0))))