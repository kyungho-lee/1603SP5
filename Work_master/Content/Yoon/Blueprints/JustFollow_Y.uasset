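; A character that trails a leader actor at a slow, fixed walk speed.
; On BeginPlay it starts a looping timer and stores the handle.
; Each tick of the timer sets the walk speed and re-issues a simple AI move toward FollowActor.
; Logic for assigning a spawn skeletal mesh and animation class is present but disconnected, so it never runs.
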(event `self.ReceiveBeginPlay`
  ;[0.9056 0.6179 1] Just Follow Leader Actor
  (bind _returnvalue (`KismetSystemLibrary.K2_SetTimerDelegate` (delegate `Follow`) 0.1 true))
  (set `self.FollowHandler` _returnvalue))

(event `Follow`
  ;[0.9056 0.6179 1] Just Follow Leader Actor
  (set `CharacterMovementComponent.MaxWalkSpeed` 70.0 (`self.CharacterMovement`))
  (`AIBlueprintHelperLibrary.SimpleMoveToActor` (`AIBlueprintHelperLibrary.GetAIController` self) (`self.FollowActor`)))

(fn `UserConstructionScript`)