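; BP_GooParticles is a goo particle jet whose reach is adjustable with the mouse wheel and which puts out fires.
; BeginPlay and wheel down shorten JetDistance by a fixed step, and wheel up lengthens it.
; Each change writes the particle vector parameter "aaa", with X as the distance and Z as negative half of it.
; When the particle component hits a BP_Fire, that fire actor is destroyed.
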(event `self.ReceiveBeginPlay`
  (bind _returnvalue (- (`self.JetDistance`) 100.0))
  (`ParticleSystemComponent.SetVectorParameter` (`self.ParticleSystem`) "aaa" (`KismetMathLibrary.MakeVector` _returnvalue 0.0 (* _returnvalue -0.5)) :!label _label)
  (set `self.JetDistance` _returnvalue))

(event `Key|MouseScrollDown` :consume false :overrideparent false
  (params (Key :type "Key Structure"))
  (:`Pressed`
    (goto _label)))

(event `Key|MouseScrollUp`
  (params (Key :type "Key Structure"))
  (bind _returnvalue (+ (`self.JetDistance`) 100.0))
  (:`Pressed`
    (`ParticleSystemComponent.SetVectorParameter` (`self.ParticleSystem`) "aaa" (`KismetMathLibrary.MakeVector` _returnvalue 0.0 (* _returnvalue -0.5)))
    (set `self.JetDistance` _returnvalue)))

(event `self.ParticleSystem.OnComponentHit`
  (params (HitComponent :type "PrimitiveComponent Object Reference") (OtherActor :type "Actor Object Reference") (OtherComp :type "PrimitiveComponent Object Reference") (NormalImpulse :type "Vector Structure") (Hit :type "HitResult Structure (by ref)"))
  (bind _asbp_fire (cast `/Game/Yoon/Blueprints/BP_Fire` OtherActor))
  (`self.K2_DestroyActor` _asbp_fire))

(event `self.ParticleSystem.OnComponentBeginOverlap`
  (params (OverlappedComponent :type "PrimitiveComponent Object Reference") (OtherActor :type "Actor Object Reference") (OtherComp :type "PrimitiveComponent Object Reference") (OtherBodyIndex :type Integer) (bFromSweep :type Boolean) (SweepResult :type "HitResult Structure (by ref)")))

(fn `UserConstructionScript`)