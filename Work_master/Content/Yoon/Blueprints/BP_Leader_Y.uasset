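; Leader actor that spawns a crowd of JustFollow characters around itself, each set to follow it, and leads them along a spline.
; A looping timer runs Patrol, which steps the leader along FollowingPath's spline only while the first JustFollow found is within a range scaled by spawn count and capsule radius.
; The timer pauses at the spline's end; path wrapping and debug drawing are left disconnected.
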(event `self.ReceiveBeginPlay`
  (while (> (`self.CharSpawn`) 0)
    ;[0.5851 1 0.4775] 팔로잉 오브젝트 스폰(설정 갯수만큼)
    (bind _returnvalue (`|SpawnActorFromClass` "/Game/CHS/02FollowPathUnit/01SimplePathMover/JustFollow.JustFollow_C" (`KismetMathLibrary.Conv_VectorToTransform` (`KismetMathLibrary.RandomPointInBoundingBox` (+ (`self.K2_GetActorLocation`) (0.0 0.0 60.0)) (300.0 300.0 50.0))) "AdjustIfPossibleButAlwaysSpawn" "OverrideRootScale" null null))
    (`SkinnedMeshComponent.SetSkinnedAssetAndUpdate` (`Character.Mesh` _returnvalue) (`self.SpawnMesh`) true)
    (`SkeletalMeshComponent.SetAnimInstanceClass` (`Character.Mesh` _returnvalue) (`self.SpawnAnimClass`))
    (`Pawn.SpawnDefaultController` _returnvalue)
    (set `/Game/CHS/02FollowPathUnit/01SimplePathMover/JustFollow.FollowActor` self _returnvalue)
    (set `self.Follower` _returnvalue)
    (`/Engine/EditorBlueprintResources/StandardMacros.DecrementInt` (`self.CharSpawn`)
      (:`  `
        (if (`KismetSystemLibrary.IsValid` _returnvalue)
          (`/Engine/EditorBlueprintResources/StandardMacros.IncrementInt` (`self.CheckSpawn`))))))
  (`KismetSystemLibrary.PrintString` (`KismetStringLibrary.Conv_IntToString` (`self.CheckSpawn`)))
  ;[0.2702 1 0.75] Leader Actor Move
  (bind _returnvalue_2 (`KismetSystemLibrary.K2_SetTimerDelegate` (delegate `Patrol`) 1.0 true))
  (set `self.PatrolHandle` _returnvalue_2))

(event `Patrol`
  (bind _follower (`self.Follower`))
  ;[0.2702 1 0.75] Leader Actor Move
  (bind _outactors (`GameplayStatics.GetAllActorsOfClass` "/Game/CHS/02FollowPathUnit/01SimplePathMover/JustFollow.JustFollow_C"))
  (bind _output (`|GetArrayItem` _outactors))
  (`/Engine/EditorBlueprintResources/StandardMacros.IsValid` _output
    (:`Is Valid`
      (set `self.Follower` _output)
      (if (<= (`KismetMathLibrary.VSizeXY` (- (`self.K2_GetActorLocation` _follower) (`self.K2_GetActorLocation`))) (* (`self.CheckSpawn`) (* 2 (`CapsuleComponent.GetScaledCapsuleRadius` (`Character.CapsuleComponent` _follower)))))
        (bind _output_get (set `self.Distance` (+ (`self.Distance`) (`self.PatrolSpeed`))))
        (if (< _output_get (`SplineComponent.GetSplineLength` (`/Game/CHS/02FollowPathUnit/01SimplePathMover/BP_SimplePath.PatrolSpline` (`self.FollowingPath`))))
          (bind _output_get_2 (set `self.TargetLocation` (`SplineComponent.GetLocationAtDistanceAlongSpline` (`/Game/CHS/02FollowPathUnit/01SimplePathMover/BP_SimplePath.PatrolSpline` (`self.FollowingPath`)) (`self.Distance`) "World")))
          (`self.K2_SetActorLocation` _output_get_2)
          (else
            (`KismetSystemLibrary.K2_PauseTimerHandle` (`self.PatrolHandle`))))))))

(fn `UserConstructionScript`)