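; Spinning blade actor that slices procedural meshes on the BP_Slice family of actors when its rotating Plane overlaps them.
; BP_Slice is cut along the blade's plane, while BP_Slice_2 and its child are cut through their own location along their right vector.
; Each branch fires once: halves get physics or pushes, BP_Slice_2 takes damage, and a child hit destroys the blade.
; Bubble and destructible logic is left unwired.
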(event `self.ReceiveTick`
  (params (DeltaSeconds :type "Float (single-precision)"))
  (`SceneComponent.K2_AddRelativeRotation` (`self.Plane`) (struct :`Yaw` 30.0) false false))

(event `self.Plane.OnComponentBeginOverlap`
  (params (OverlappedComponent :type "PrimitiveComponent Object Reference") (OtherActor :type "Actor Object Reference") (OtherComp :type "PrimitiveComponent Object Reference") (OtherBodyIndex :type Integer) (bFromSweep :type Boolean) (SweepResult :type "HitResult Structure (by ref)"))
  (bind _plane (`self.Plane`))
  (`|ExecutionSequence`
    (:`then_0`
      (cast `/Game/Yoon/Blueprints/BP_Slice` OtherActor)
      (bind _asprocedural_mesh_component (cast `ProceduralMeshComponent` OtherComp))
      (`/Engine/EditorBlueprintResources/StandardMacros.DoOnce` false
        (:`Completed`
          (bind _outotherhalfprocmesh (`KismetProceduralMeshLibrary.SliceProceduralMesh` _asprocedural_mesh_component (`SceneComponent.K2_GetComponentLocation` _plane) (`SceneComponent.GetUpVector` _plane) true "CreateNewSectionForCap" "/Engine/VREditor/UI/ArrowMaterial.ArrowMaterial"))
          (`PrimitiveComponent.SetSimulatePhysics` _outotherhalfprocmesh true)
          (`KismetSystemLibrary.Delay` 3.0)
          (`PrimitiveComponent.SetSimulatePhysics` _outotherhalfprocmesh true))))
    (:`then_5`
      (bind _asbp_slice_2_child (cast `/Game/Yoon/Blueprints/BP_Slice_2_Child` (`.HitActor` (`GameplayStatics.BreakHitResult` SweepResult))))
      (bind _asprocedural_mesh_component_2 (cast `ProceduralMeshComponent` OtherComp))
      (`/Engine/EditorBlueprintResources/StandardMacros.DoOnce` false
        (:`Completed`
          (bind _outotherhalfprocmesh_2 (`KismetProceduralMeshLibrary.SliceProceduralMesh` _asprocedural_mesh_component_2 (`self.K2_GetActorLocation` _asbp_slice_2_child) (`SceneComponent.GetRightVector` (`/Game/Yoon/Blueprints/BP_Slice_2.ProceduralMesh` _asbp_slice_2_child)) true "CreateNewSectionForCap" "/Game/Art/PolygonAdventure/BP_obstacle/NewMaterial.NewMaterial"))
          (`self.K2_DestroyActor`)
          (bind _proceduralmesh (`/Game/Yoon/Blueprints/BP_Slice_2.ProceduralMesh` _asbp_slice_2_child))
          (`PrimitiveComponent.SetSimulatePhysics` _proceduralmesh true)
          (`PrimitiveComponent.AddForce` _proceduralmesh (0.0 0.0 -1000.0) "None" true)
          (`GameplayStatics.ApplyDamage` null 1.0))))
    (:`then_6`
      (bind _asbp_slice_2 (cast `/Game/Yoon/Blueprints/BP_Slice_2` OtherActor))
      (bind _asprocedural_mesh_component_3 (cast `ProceduralMeshComponent` OtherComp))
      (`/Engine/EditorBlueprintResources/StandardMacros.DoOnce` false
        (:`Completed`
          (bind _returnvalue (`SceneComponent.GetRightVector` (`/Game/Yoon/Blueprints/BP_Slice_2.ProceduralMesh` _asbp_slice_2)))
          (bind _outotherhalfprocmesh_3 (`KismetProceduralMeshLibrary.SliceProceduralMesh` _asprocedural_mesh_component_3 (`self.K2_GetActorLocation` _asbp_slice_2) _returnvalue true "CreateNewSectionForCap" "/Game/00Final/03Resource/animal/PolarBear/ANIMAL-BROWN1.ANIMAL-BROWN1"))
          (`PrimitiveComponent.SetSimulatePhysics` _outotherhalfprocmesh_3 true)
          (bind _returnvalue_2 (* _returnvalue 500.0))
          (`PrimitiveComponent.AddImpulse` _outotherhalfprocmesh_3 (* _returnvalue_2 -1.0) "None" true)
          (`PrimitiveComponent.AddImpulse` _asprocedural_mesh_component_3 _returnvalue_2 "None" true)
          (`GameplayStatics.ApplyDamage` _asbp_slice_2 10.0))))))

(fn `UserConstructionScript`)