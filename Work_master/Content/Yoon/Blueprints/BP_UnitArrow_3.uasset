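; BP_UnitArrow_3 is an arrow actor that switches between three orientations when clicked.
; ClickArrow cycles the Click state through three values, setting the relative rotation to 0, -90 or -180 degrees on one axis.
; SetNum overrides Click with a given number, then resets it to zero after a ten-second delay, without changing the rotation itself.
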(event `ClickArrow`
  (switch `int` (`self.Click`)
    (:`0`
      (set `self.Click` 1)
      (`self.K2_SetActorRelativeRotation` (struct :`Yaw` -90.0)))
    (:`1`
      (set `self.Click` 2)
      (`self.K2_SetActorRelativeRotation` (struct :`Yaw` -180.0)))
    (:`2`
      (set `self.Click` 0)
      (`self.K2_SetActorRelativeRotation` (struct)))))

(event `SetNum`
  (params (Number :type Integer))
  (set `self.Click` Number)
  (`KismetSystemLibrary.Delay` 10.0)
  (set `self.Click` 0))

(fn `UserConstructionScript`)