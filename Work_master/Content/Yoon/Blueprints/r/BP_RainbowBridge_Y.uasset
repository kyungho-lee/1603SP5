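; Rainbow bridge actor that moves into position and animates its opacity when its Boom event is called.
; A timeline lerps the Bridge component's relative location from Start to End.
; A delay chained off that timeline's update creates a dynamic rainbow material instance on the bridge, then plays a second timeline.
; That timeline drives the material's Opacity parameter.
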(event `/Game/Art/Hemi/BluePrints/BPI_Boom.Boom`
  (bind (_direction _newtrack_0) (`Timeline|Timeline_1`)
    (:`Update`
      (`SceneComponent.K2_SetRelativeLocation` (`self.Bridge`) (`KismetMathLibrary.VLerp` (`self.start`) (`self.end`) _newtrack_0) false false)
      (`KismetSystemLibrary.Delay` 1.5)
      (bind _returnvalue (`PrimitiveComponent.CreateDynamicMaterialInstance` (`self.Bridge`) 0 "/Game/Art/PolygonAdventure/BP_obstacle/MT_Rainbow1_Inst.MT_Rainbow1_Inst" "None"))
      (bind (_direction_2 _newtrack_0_2) (`Timeline|Timeline_0`)
        (:`Update`
          (`MaterialInstanceDynamic.SetScalarParameterValue` _returnvalue "Opacity" _newtrack_0_2))))))

(fn `UserConstructionScript`)