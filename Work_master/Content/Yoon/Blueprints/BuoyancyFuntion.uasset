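; Buoyancy function that makes a physics component float by pushing it off a surface detected beneath it.
; A downward line trace, sized by BuoyancyStart plus average world scale, searches a fixed object type, leaving the CollisionChannel input unused.
; On a hit, it applies mass-scaled force along the impact normal, fading with distance via a Lerp over BuoyancyStart, and sets light linear and angular damping.
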(fn `Buoyancy Function`
  (params (PhysicsComponentToFloat :type "PrimitiveComponent Object Reference") (BuoyancyStart :type "Float (double-precision)") (CollisionChannel :type "EObjectTypeQuery Enum" :default "ObjectTypeQuery1"))
  (bind _returnvalue (`SceneComponent.K2_GetComponentLocation` PhysicsComponentToFloat))
  (bind (_returnvalue_x _returnvalue_y _returnvalue_z) (`KismetMathLibrary.BreakVector` (`SceneComponent.K2_GetComponentScale` PhysicsComponentToFloat)))
  (bind (_outhit _returnvalue_2) (`KismetSystemLibrary.LineTraceSingleForObjects` null _returnvalue (- _returnvalue (`KismetMathLibrary.MakeVector` 0.0 0.0 (+ (/ (+ _returnvalue_x _returnvalue_y _returnvalue_z) 3.0) BuoyancyStart))) (`|MakeArray` "ObjectTypeQuery7" :!type "EObjectTypeQuery Enum")))
  (if _returnvalue_2
    (bind (_bblockinghit _binitialoverlap _time _distance _location _impactpoint _normal _impactnormal) (`GameplayStatics.BreakHitResult` _outhit))
    (`PrimitiveComponent.AddForce` PhysicsComponentToFloat (* _impactnormal (`KismetMathLibrary.Lerp` (* (`PrimitiveComponent.GetMass` PhysicsComponentToFloat) 6000.0) 0.0 (/ (`KismetMathLibrary.VSize` (- _location (`SceneComponent.K2_GetComponentLocation` PhysicsComponentToFloat))) (* BuoyancyStart 1.0)))) "None" false)
    (`PrimitiveComponent.SetLinearDamping` PhysicsComponentToFloat 0.1)
    (`PrimitiveComponent.SetAngularDamping` PhysicsComponentToFloat 0.1)))