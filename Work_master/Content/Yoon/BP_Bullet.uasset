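; BP_Bullet is a short-lived bullet actor that destroys itself after a few seconds and reacts to whatever its Plane component overlaps.
; The first procedural mesh hit is sliced along the plane, with the new half simulating physics and the original receiving a radial impulse.
; BP_Target actors get their DoSomething call.
; BP_Destruction actors receive radial damage and an impulse on their destructible component.
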(event `self.ReceiveBeginPlay`
  (`self.SetLifeSpan` 5.0))

(event `self.Plane.OnComponentBeginOverlap`
  (params (OverlappedComponent :type "PrimitiveComponent Object Reference") (OtherActor :type "Actor Object Reference") (OtherComp :type "PrimitiveComponent Object Reference") (OtherBodyIndex :type Integer) (bFromSweep :type Boolean) (SweepResult :type "HitResult Structure (by ref)"))
  (bind _plane (`self.Plane`))
  (bind _returnvalue (`SceneComponent.GetUpVector` _plane))
  (`|ExecutionSequence`
    (:`then_0`
      (bind _asprocedural_mesh_component (cast `ProceduralMeshComponent` OtherComp))
      (`/Engine/EditorBlueprintResources/StandardMacros.DoOnce` false
        (:`Completed`
          (bind _outotherhalfprocmesh (`KismetProceduralMeshLibrary.SliceProceduralMesh` _asprocedural_mesh_component (`SceneComponent.K2_GetComponentLocation` _plane) _returnvalue true "UseLastSectionForCap" "/Engine/MapTemplates/Materials/BasicAsset01.BasicAsset01"))
          (`PrimitiveComponent.SetSimulatePhysics` _outotherhalfprocmesh true)
          (`PrimitiveComponent.AddRadialImpulse` _asprocedural_mesh_component _returnvalue 600.0 500.0 "RIF_Constant" true))))
    (:`then_1`
      (bind _asbp_target (cast `/Game/Yoon/BP_Target` OtherActor))
      (`/Game/Yoon/BP_Target.DoSomething` _asbp_target))
    (:`then_2`
      (bind _asbp_destruction (cast `/Game/Yoon/BP_Destruction` OtherActor))
      (bind _returnvalue_2 (`self.K2_GetActorLocation` _asbp_destruction))
      (`GameplayStatics.ApplyRadialDamage` :`BaseDamage` 10.0 :`Origin` _returnvalue_2 :`DamageRadius` 5.0 :`DamageCauser` null :`InstigatedByController` null)
      (`PrimitiveComponent.AddRadialImpulse` (`/Game/Yoon/BP_Destruction.Destructible` _asbp_destruction) _returnvalue_2 100.0 1000.0 "RIF_Constant" true))))

(fn `UserConstructionScript`)