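; BP_Fire is a self-propagating fire actor that spreads forward in a chain of explosions and is destroyed by goo particles.
; On BeginPlay it spawns an explosion emitter, then after a short delay spawns another BP_Fire ahead along its forward vector.
; DontSpawnIfColliding halts the chain when the next spot is blocked.
; Its box collision destroys it on any hit or on overlap with GooParticles_BP.
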(event `self.ReceiveBeginPlay`
  (bind (_returnvalue_location _returnvalue_rotation _returnvalue_scale) (`KismetMathLibrary.BreakTransform` (`self.GetTransform`)))
  (bind (_returnvalue_location_2 _returnvalue_rotation_2 _returnvalue_scale_2) (`KismetMathLibrary.BreakTransform` (`self.GetTransform`)))
  (`GameplayStatics.SpawnEmitterAtLocation` "/Game/UnrealDefaultAsset/StarterContent/Particles/P_Explosion.P_Explosion" _returnvalue_location _returnvalue_rotation _returnvalue_scale true "AutoRelease")
  (`KismetSystemLibrary.Delay` 0.8)
  (`|SpawnActorFromClass` "BP_Fire_C" (`KismetMathLibrary.MakeTransform` (+ _returnvalue_location_2 (* (`self.GetActorForwardVector`) 100.0)) _returnvalue_rotation_2 _returnvalue_scale_2) "DontSpawnIfColliding" "OverrideRootScale" null null))

(event `self.BoxCollision.OnComponentBeginOverlap`
  (params (OverlappedComponent :type "PrimitiveComponent Object Reference") (OtherActor :type "Actor Object Reference") (OtherComp :type "PrimitiveComponent Object Reference") (OtherBodyIndex :type Integer) (bFromSweep :type Boolean) (SweepResult :type "HitResult Structure (by ref)"))
  (cast `/Game/Yoon/_Marvelmaster_infinite_reactive_water_/Blueprints/GooParticles_BP` OtherActor)
  (`self.K2_DestroyActor`))

(event `self.BoxCollision.OnComponentHit`
  (params (HitComponent :type "PrimitiveComponent Object Reference") (OtherActor :type "Actor Object Reference") (OtherComp :type "PrimitiveComponent Object Reference") (NormalImpulse :type "Vector Structure") (Hit :type "HitResult Structure (by ref)"))
  (`self.K2_DestroyActor`))

(fn `UserConstructionScript`)