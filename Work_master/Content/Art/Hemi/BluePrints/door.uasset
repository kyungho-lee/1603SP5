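; Interactable door Blueprint that slides its static mesh between a start and an end location.
; Each Interact call flips InteractState and plays or reverses a timeline.
; The timeline's DoorSpeed track drives a vector lerp that sets the mesh's relative location, without sweep.
; GetInteract exposes the current toggle state.
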(event `/Game/Art/Hemi/BluePrints/bPI_interactable.interact`
  (if (`self.interactState`)
    (set `self.interactState` false)
    (bind (_direction _doorspeed) (`Timeline|Timeline_0` :!via `Reverse` :!label _label)
      (:`Update`
        (`SceneComponent.K2_SetRelativeLocation` (`self.StaticMesh`) (`KismetMathLibrary.VLerp` (`self.StartLocation`) (`self.EndLocation`) _doorspeed) false false)))
    (else
      (set `self.interactState` true)
      (goto _label))))

(fn `getInteract`
  (returns (interactState :type Boolean))
  (return (`self.interactState`)))

(fn `UserConstructionScript`)