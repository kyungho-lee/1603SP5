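; BP_BoxScatter is a level design tool that scatters random static meshes onto surfaces beneath a box volume.
; The construction script repeatedly traces between random points in the box, offsetting the end downward, and adds a manually attached mesh component at each impact point.
; Yaw and per-axis scale variation use a seeded stream, while trace points and mesh choice from MeshesToSpawn are unseeded.
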(fn `UserConstructionScript`
  (bind _box (`self.Box`))
  (bind _meshes_to_spawn (`self.Meshes to spawn`))
  (bind _seed (`self.Seed`))
  (bind _setplacementscale (`self.SetPlacementScale`))
  (bind _returnvalue (`KismetMathLibrary.RandomFloatInRangeFromStream` 0.9 1.1 _seed))
  (bind _returnvalue_2 (`KismetMathLibrary.RandomPointInBoundingBox` (`SceneComponent.K2_GetComponentLocation` _box) (`BoxComponent.BoxExtent` _box)))
  (bind _output_get (set `self.Number of meshes` (`KismetMathLibrary.Clamp` (`self.Number of meshes`) 1 50))) ; Clamp value so it can't be 0
  (for _ (range 1 (+ _output_get 1))
    (`BoxComponent.SetBoxExtent` (`self.Box`) (`KismetMathLibrary.MakeVector` _setplacementscale _setplacementscale 150.0) true)
    (bind _outhit (`KismetSystemLibrary.LineTraceSingle` :`Start` (+ _returnvalue_2 (0.0 0.0 0.0)) :`End` (+ _returnvalue_2 (0.0 0.0 -1500.0)) :`TraceChannel` "TraceTypeQuery1" :`bTraceComplex` true :`DrawDebugType` "Persistent" :`bIgnoreSelf` false))
    (bind _returnvalue_3 (`AddComponent|NODE_AddStaticMeshComponent-3` :`bManualAttachment` true :`RelativeTransform` (`KismetMathLibrary.MakeTransform` (`.ImpactPoint` (`GameplayStatics.BreakHitResult` _outhit)) (`KismetMathLibrary.MakeRotator` 0.0 0.0 (`KismetMathLibrary.RandomFloatInRangeFromStream` -170.0 170.0 _seed)) (`KismetMathLibrary.MakeVector` _returnvalue _returnvalue _returnvalue))))
    (`StaticMeshComponent.SetStaticMesh` _returnvalue_3 (`|GetArrayItem` _meshes_to_spawn (`KismetMathLibrary.RandomIntegerInRange` 0 (`KismetArrayLibrary.Array_LastIndex` _meshes_to_spawn)))) ; Change the new static mesh to the specified type
  ))