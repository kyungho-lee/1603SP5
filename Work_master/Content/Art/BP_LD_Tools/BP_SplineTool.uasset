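; BP_SplineTool is a level design tool that places a selected mesh along a spline at regular spacing.
; Its construction script steps along the spline, adding Hierarchical Instanced Static Mesh instances.
; With UseRandom on, line traces set each instance's height, and a seeded stream randomizes yaw and scale.
; Otherwise, instances sit on the spline, rotated from their world location vector rather than its tangent, with yaw multiplied by AddRotation.
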(fn `UserConstructionScript`
  (bind _seed (`self.Seed`))
  (bind _nextdistance (`self.NextDistance`))
  (bind _returnvalue (`SplineComponent.GetLocationAtDistanceAlongSpline` (`self.Spline`) _nextdistance "World"))
  (bind _returnvalue_2 (`KismetMathLibrary.RandomFloatInRangeFromStream` 0.9 1.1 _seed))
  (bind _returnvalue_3 (`SplineComponent.GetLocationAtDistanceAlongSpline` (`self.Spline`) _nextdistance "World"))
  (bind _selectmesh (`self.SelectMesh`)
    (:`then`
      (`StaticMeshComponent.SetStaticMesh` (`self.HierarchicalInstancedStaticMesh`) _selectmesh)
      (while (<= _nextdistance (`SplineComponent.GetSplineLength` (`self.Spline`)))
        (if (`self.UseRandom`)
          (bind _outhit (`KismetSystemLibrary.LineTraceSingle` (+ _returnvalue_3 (0.0 0.0 250.0)) (+ _returnvalue_3 (0.0 0.0 -500.0)) "TraceTypeQuery1" true))
          (`InstancedStaticMeshComponent.AddInstanceWorldSpace` (`self.HierarchicalInstancedStaticMesh`) (`KismetMathLibrary.MakeTransform` (`KismetMathLibrary.MakeVector` (.x _returnvalue_3) (.y _returnvalue_3) (.z (`.Location` (`GameplayStatics.BreakHitResult` _outhit)))) (`KismetMathLibrary.MakeRotator` 0.0 0.0 (`KismetMathLibrary.RandomFloatInRangeFromStream` -170.0 170.0 _seed)) (`KismetMathLibrary.MakeVector` _returnvalue_2 _returnvalue_2 _returnvalue_2)))
          (set `self.NextDistance` (+ (`self.Spacing`) (`self.NextDistance`)))
          (else
            (`InstancedStaticMeshComponent.AddInstanceWorldSpace` (`self.HierarchicalInstancedStaticMesh`) (`KismetMathLibrary.MakeTransform` _returnvalue (`KismetMathLibrary.MakeRotator` (.roll (`KismetMathLibrary.Conv_VectorToRotator` _returnvalue)) (.pitch (`KismetMathLibrary.Conv_VectorToRotator` _returnvalue)) (* (.yaw (`KismetMathLibrary.Conv_VectorToRotator` _returnvalue)) (`self.AddRotation`)))))
            (set `self.NextDistance` (+ (`self.Spacing`) (`self.NextDistance`)))))))
    (:`else`)))