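; Level-design tool that procedurally builds a brick wall from a single mesh on a rows-by-columns grid.
; The construction script offsets alternate rows and adds seeded position and rotation jitter, with optional random quarter-turns per axis.
; Bricks become either separate static mesh components or hierarchical instanced mesh instances, depending on a toggle.
; CreateStaticMeshes spawns a standalone, labeled StaticMeshActor at each brick's transform.
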(event `CreateStaticMeshes`
  (bind _brickmesh (`self.BrickMesh`))
  (bind _brickmesh_2 (`self.BrickMesh`))
  (bind _hierarchicalinstancedstaticmesh (`self.HierarchicalInstancedStaticMesh`))
  (if (`self.UseStaticMeshes`)
    (for _array_element (`SceneComponent.GetChildrenComponents` (`self.DefaultSceneRoot`) true)
      (bind _returnvalue (`|SpawnActorFromClass` "/Script/Engine.StaticMeshActor" (`SceneComponent.K2_GetComponentToWorld` _array_element) "AlwaysSpawn" "OverrideRootScale" null null))
      (`self.SetActorLabel` _returnvalue (`KismetSystemLibrary.GetObjectName` _brickmesh) true)
      (`StaticMeshComponent.SetStaticMesh` (`StaticMeshActor.StaticMeshComponent` _returnvalue) _brickmesh))
    (else
      (for _index (range (`InstancedStaticMeshComponent.GetInstanceCount` _hierarchicalinstancedstaticmesh))
        (bind _returnvalue_2 (`|SpawnActorFromClass` "/Script/Engine.StaticMeshActor" (`InstancedStaticMeshComponent.GetInstanceTransform` _hierarchicalinstancedstaticmesh _index true) "AlwaysSpawn" "OverrideRootScale" null null))
        (`self.SetActorLabel` _returnvalue_2 (`KismetSystemLibrary.GetObjectName` _brickmesh_2) true)
        (`StaticMeshComponent.SetStaticMesh` (`StaticMeshActor.StaticMeshComponent` _returnvalue_2) _brickmesh_2)))))

(fn `UserConstructionScript`
  (locals (RandomNum :type "Float (double-precision)" :default 0.0) (RandomInt :type Integer :default 0))
  (bind _brickscale (`self.BrickScale`))
  (bind (_returnvalue_x _returnvalue_y _returnvalue_z) (`KismetMathLibrary.BreakVector` (* (`self.RandomPosition`) (`local.RandomNum`))))
  (bind _returnvalue (* (`local.RandomInt`) 90.0))
  (bind (_returnvalue_roll _returnvalue_pitch _returnvalue_yaw) (`KismetMathLibrary.BreakRotator` (* (`self.RandomRotation`) (`local.RandomNum`))))
  (bind _returnvalue_2 (`KismetMathLibrary.SelectFloat` (+ _returnvalue _returnvalue_roll) _returnvalue_roll (`self.Randomize Orientation Roll`)))
  (bind _returnvalue_3 (`KismetMathLibrary.SelectFloat` (+ _returnvalue _returnvalue_pitch) _returnvalue_pitch (`self.Randomize Orientation Pitch`)))
  (bind _returnvalue_4 (`KismetMathLibrary.SelectFloat` (+ _returnvalue _returnvalue_yaw) _returnvalue_yaw (`self.Randomize Orientation Yaw`)))
  (`self.BrickMesh`
    (:`then`
      (if (not (`self.UseStaticMeshes`))
        (`StaticMeshComponent.SetStaticMesh` (`self.HierarchicalInstancedStaticMesh`) (`self.BrickMesh`)))
      (for _index (range (+ (`KismetMathLibrary.Max` (- (`self.InstancesVertical`) 1)) 1))
        (for _index_2 (range (+ (`KismetMathLibrary.Max` (- (`self.InstancesHorizontal`) 1)) 1))
          (set `local.RandomNum` (`KismetMathLibrary.RandomFloatInRangeFromStream` -1.0 1.0 (`self.RandomStream`)))
          (set `local.RandomInt` (`KismetMathLibrary.RandomIntegerFromStream` 4 (`self.RandomStream`)))
          (if (`self.UseStaticMeshes`)
            (bind _returnvalue_5 (+ (* _index_2 (`self.SpacingHorizontal`)) (select `bool` (> (mod _index 2) 0) :`true` (`self.HorizontalShift`)) _returnvalue_y))
            (bind _returnvalue_6 (+ (* _index (`self.SpacingVertical`)) _returnvalue_z))
            (bind _returnvalue_7 (`AddComponent|NODE_AddStaticMeshComponent-0` :`RelativeTransform` (`KismetMathLibrary.MakeTransform` (`KismetMathLibrary.MakeVector` _returnvalue_x _returnvalue_5 _returnvalue_6) (`KismetMathLibrary.MakeRotator` _returnvalue_2 _returnvalue_3 _returnvalue_4) _brickscale)))
            (`StaticMeshComponent.SetStaticMesh` _returnvalue_7 (`self.BrickMesh`))
            (else
              (`InstancedStaticMeshComponent.AddInstance` (`self.HierarchicalInstancedStaticMesh`) (`KismetMathLibrary.MakeTransform` (`KismetMathLibrary.MakeVector` _returnvalue_x _returnvalue_5 _returnvalue_6) (`KismetMathLibrary.MakeRotator` _returnvalue_2 _returnvalue_3 _returnvalue_4) _brickscale)))))))
    (:`else`)))