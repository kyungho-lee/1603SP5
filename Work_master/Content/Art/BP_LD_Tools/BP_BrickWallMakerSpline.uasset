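; Level-design tool that builds a procedural brick wall from BrickMesh along a spline.
; The construction script lays rows and columns by spline distance, shifting alternate rows and applying seeded random offsets, rotations and angle-locked orientation flips, optionally following spline rotation.
; Bricks become either HISM instances or individual StaticMeshComponents, depending on UseStaticMeshes.
; CreateStaticMeshes bakes the result by spawning a separate, labeled StaticMeshActor at each brick's world transform.
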(event `CreateStaticMeshes`
  (bind _brickmesh (`self.BrickMesh`))
  (bind _brickmesh_2 (`self.BrickMesh`))
  (bind _hierarchicalinstancedstaticmesh (`self.HierarchicalInstancedStaticMesh`))
  (if (`self.UseStaticMeshes`)
    (for _array_element (`SceneComponent.GetChildrenComponents` (`self.DefaultSceneRoot`) true)
      (bind _returnvalue (`|SpawnActorFromClass` "/Script/Engine.StaticMeshActor" (`SceneComponent.K2_GetComponentToWorld` _array_element) "AlwaysSpawn" "OverrideRootScale" null null))
      (`self.SetActorLabel` _returnvalue (`KismetSystemLibrary.GetObjectName` _brickmesh) true)
      (`StaticMeshComponent.SetStaticMesh` (`StaticMeshActor.StaticMeshComponent` _returnvalue) _brickmesh))
    (else
      (for _index (range (`InstancedStaticMeshComponent.GetInstanceCount` _hierarchicalinstancedstaticmesh))
        (bind _returnvalue_2 (`|SpawnActorFromClass` "/Script/Engine.StaticMeshActor" (`InstancedStaticMeshComponent.GetInstanceTransform` _hierarchicalinstancedstaticmesh _index true) "AlwaysSpawn" "OverrideRootScale" null null))
        (`self.SetActorLabel` _returnvalue_2 (`KismetSystemLibrary.GetObjectName` _brickmesh_2) true)
        (`StaticMeshComponent.SetStaticMesh` (`StaticMeshActor.StaticMeshComponent` _returnvalue_2) _brickmesh_2)))))

(fn `UserConstructionScript`
  (locals (RandomNum :type "Float (double-precision)" :default 0.0) (RandomInt :type Integer :default 0))
  (bind (_basetranform_location _basetranform_rotation _basetranform_scale) (`KismetMathLibrary.BreakTransform` (`self.BaseTranform`)))
  (bind _basetranform_location_2 (`KismetMathLibrary.BreakTransform` (`self.BaseTranform`)))
  (bind _spline (`self.Spline`))
  (bind _followsplinerotation (`self.FollowSplineRotation`))
  (bind (_basetranform_location_3 _basetranform_rotation_2) (`KismetMathLibrary.BreakTransform` (`self.BaseTranform`)))
  (bind _returnvalue (* (`local.RandomInt`) (`self.AngleLock`)))
  (bind _returnvalue_2 (`KismetMathLibrary.ComposeRotators` (`KismetMathLibrary.ComposeRotators` _basetranform_rotation_2 (* (`self.RandomRotation`) (`local.RandomNum`))) (`KismetMathLibrary.MakeRotator` (* _returnvalue (`KismetMathLibrary.Conv_BoolToDouble` (`self.Randomize Orientation Roll`))) (* _returnvalue (`KismetMathLibrary.Conv_BoolToDouble` (`self.Randomize Orientation Pitch`))) (* _returnvalue (`KismetMathLibrary.Conv_BoolToDouble` (`self.Randomize Orientation Yaw`))))))
  (`self.BrickMesh`
    (:`then`
      (if (not (`self.UseStaticMeshes`))
        (`StaticMeshComponent.SetStaticMesh` (`self.HierarchicalInstancedStaticMesh`) (`self.BrickMesh`)))
      (for _index (range (+ (`KismetMathLibrary.Max` (- (`self.InstancesVertical`) 1)) 1))
        (for _index_2 (range (+ (`KismetMathLibrary.Max` (- (`self.InstancesHorizontal`) 1)) 1))
          (set `local.RandomNum` (`KismetMathLibrary.RandomFloatInRangeFromStream` -1.0 1.0 (`self.RandomStream`)))
          (set `local.RandomInt` (`KismetMathLibrary.RandomIntegerFromStream` 4 (`self.RandomStream`)))
          (if (`self.UseStaticMeshes`)
            (bind _returnvalue_3 (* _index_2 (`self.SpacingHorizontal`)))
            (bind (_returnvalue_x _returnvalue_y _returnvalue_z) (`KismetMathLibrary.BreakVector` (+ (select `bool` (> (mod _index 2) 0) :`true` (`self.AlternatingShift`)) (* (`self.RandomPosition`) (`local.RandomNum`)) _basetranform_location_2)))
            (bind _returnvalue_4 (`KismetMathLibrary.MakeVector` 0.0 _returnvalue_y (+ (* _index (`self.SpacingVertical`)) _returnvalue_z)))
            (bind _returnvalue_5 (`SplineComponent.GetTransformAtDistanceAlongSpline` _spline _returnvalue_3 "Local" false))
            (bind (_returnvalue_x_2 _returnvalue_y_2 _returnvalue_z_2) (`KismetMathLibrary.BreakVector` (select `bool` _followsplinerotation :`false` (`KismetMathLibrary.TransformLocation` (`KismetMathLibrary.MakeTransform` (`SplineComponent.GetLocationAtDistanceAlongSpline` _spline _returnvalue_3 "Local")) _returnvalue_4) :`true` (`KismetMathLibrary.TransformLocation` _returnvalue_5 _returnvalue_4))))
            (bind (_returnvalue_roll _returnvalue_pitch _returnvalue_yaw) (`KismetMathLibrary.BreakRotator` (select `bool` _followsplinerotation :`false` _returnvalue_2 :`true` (`KismetMathLibrary.TransformRotation` _returnvalue_5 _returnvalue_2))))
            (bind _returnvalue_6 (`AddComponent|NODE_AddStaticMeshComponent-0` :`RelativeTransform` (`KismetMathLibrary.MakeTransform` (`KismetMathLibrary.MakeVector` _returnvalue_x_2 _returnvalue_y_2 _returnvalue_z_2) (`KismetMathLibrary.MakeRotator` _returnvalue_roll _returnvalue_pitch _returnvalue_yaw) _basetranform_scale)))
            (`StaticMeshComponent.SetStaticMesh` _returnvalue_6 (`self.BrickMesh`))
            (else
              (`InstancedStaticMeshComponent.AddInstance` (`self.HierarchicalInstancedStaticMesh`) (`KismetMathLibrary.MakeTransform` (`KismetMathLibrary.MakeVector` _returnvalue_x_2 _returnvalue_y_2 _returnvalue_z_2) (`KismetMathLibrary.MakeRotator` _returnvalue_roll _returnvalue_pitch _returnvalue_yaw) _basetranform_scale)))))))
    (:`else`)))