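; BP_SplineContentSample is a sample spline tool that places a set number of static meshes evenly along its spline.
; The construction script adds one uniformly scaled mesh component per count, spacing them by spline length over count minus one so they span both ends.
; World-space spline locations are converted to actor-relative transforms, and OrientToSpline optionally rotates each mesh to follow the spline direction.
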(fn `UserConstructionScript`
  (bind _number_of_meshes (`self.Number of meshes`))
  (bind _returnvalue (- _number_of_meshes 1))
  (if (> _number_of_meshes 0)
    (for _index (range (+ _returnvalue 1))
      (bind _returnvalue_2 (* _index (/ (`SplineComponent.GetSplineLength` (`self.Spline`)) (`KismetMathLibrary.Conv_IntToDouble` _returnvalue))))
      (bind _returnvalue_3 (`AddComponent|NODE_AddStaticMeshComponent-0` :`RelativeTransform` (`KismetMathLibrary.MakeTransform` (`KismetMathLibrary.InverseTransformLocation` (`self.GetTransform`) (`SplineComponent.GetLocationAtDistanceAlongSpline` (`self.Spline`) _returnvalue_2 "World")) (struct) (0.6 0.6 0.6)))) ; Add static mesh component
      (if (`self.Orient to spline`)
        (`SceneComponent.K2_SetWorldRotation` _returnvalue_3 (`SplineComponent.GetRotationAtDistanceAlongSpline` (`self.Spline`) _returnvalue_2 "World") false false) ; Rotate mesh to match direction of spline at its position
      ))))