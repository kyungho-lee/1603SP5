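; BP_AI is a leader character that walks a spline path with a group of spawned JustFollow followers.
; On BeginPlay it spawns CharSpawn followers with controllers nearby, each targeting the leader.
; A one-second looping timer advances a goal along the spline for SimpleMoveToLocation, only while the last spawned follower is within a radius scaled by group size.
; The timer pauses at path end or on TriggerBox overlap; bridge resume logic is unconnected.
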(event `self.ReceiveBeginPlay`
  (while (> (`self.CharSpawn`) 0)
    ;[0.5851 1 0.4775] 팔로잉 오브젝트 스폰(설정 갯수만큼)
    (bind _returnvalue (`|SpawnActorFromClass` "/Game/CHS/02FollowPathUnit/01SimplePathMover/JustFollow.JustFollow_C" (`KismetMathLibrary.Conv_VectorToTransform` (`KismetMathLibrary.RandomPointInBoundingBox` (`self.K2_GetActorLocation`) (100.0 100.0 50.0))) "AdjustIfPossibleButAlwaysSpawn" "OverrideRootScale" null null))
    (`self.SpawnDefaultController` _returnvalue)
    (set `/Game/CHS/02FollowPathUnit/01SimplePathMover/JustFollow.FollowActor` self _returnvalue)
    (set `self.Follower` _returnvalue)
    (`/Engine/EditorBlueprintResources/StandardMacros.DecrementInt` (`self.CharSpawn`)
      (:`  `
        (if (`KismetSystemLibrary.IsValid` _returnvalue)
          (`/Engine/EditorBlueprintResources/StandardMacros.IncrementInt` (`self.CheckSpawn`))))))
  (`KismetSystemLibrary.PrintString` (`KismetStringLibrary.Conv_IntToString` (`self.CheckSpawn`)))
  ;[0.2702 1 0.75] Leader Actor Move
  (bind _returnvalue_2 (`KismetSystemLibrary.K2_SetTimerDelegate` (delegate `Patrol`) 1.0 true))
  (set `self.PatrolHandle` _returnvalue_2))

(event `Patrol`
  (bind _returnvalue (`self.K2_GetActorLocation`))
  (bind _follower (`self.Follower`))
  (bind _returnvalue_2 (`self.K2_GetActorLocation` _follower))
  ;[0.2702 1 0.75] Leader Actor Move
  (if (<= (`KismetMathLibrary.VSizeXY` (- _returnvalue_2 _returnvalue)) (* (`self.CheckSpawn`) (* 2 (`CapsuleComponent.GetScaledCapsuleRadius` (`Character.CapsuleComponent` _follower)))))
    ;[1 0.09555 0] ForDebug
    (`KismetSystemLibrary.DrawDebugLine` _returnvalue_2 _returnvalue (struct :`R` 1.0 :`B` 0.035682 :`A` 1.0) 3.0 3.0)
    (bind _output_get (set `self.Distance` (+ (`self.Distance`) (`self.PatrolSpeed`))))
    (if (< _output_get (`SplineComponent.GetSplineLength` (`/Game/CHS/02FollowPathUnit/01SimplePathMover/BP_SimplePath.PatrolSpline` (`self.FollowingPath`))))
      ;[1 0.2462 0.06393] For Debug
      (`KismetSystemLibrary.LineTraceSingle` :`Start` (stale _output_get_2) :`End` (`KismetMathLibrary.MakeVector` (.x (stale _output_get_2)) (.y (stale _output_get_2)) (+ (.z (stale _output_get_2)) 500.0)) :`TraceChannel` "TraceTypeQuery1" :`DrawDebugType` "ForDuration" :`DrawTime` 0.5)
      (bind _output_get_2 (set `self.TargetLocation` (`SplineComponent.GetLocationAtDistanceAlongSpline` (`/Game/CHS/02FollowPathUnit/01SimplePathMover/BP_SimplePath.PatrolSpline` (`self.FollowingPath`)) (`self.Distance`) "World")))
      (`AIBlueprintHelperLibrary.SimpleMoveToLocation` (`self.GetController`) _output_get_2)
      (else
        (`KismetSystemLibrary.K2_PauseTimerHandle` (`self.PatrolHandle`))))))

(event `self.CapsuleComponent.OnComponentBeginOverlap`
  (params (OverlappedComponent :type "PrimitiveComponent Object Reference") (OtherActor :type "Actor Object Reference") (OtherComp :type "PrimitiveComponent Object Reference") (OtherBodyIndex :type Integer) (bFromSweep :type Boolean) (SweepResult :type "HitResult Structure (by ref)"))
  (`|ExecutionSequence`
    (:`then_0`
      (cast `TriggerBox` OtherActor)
      (`KismetSystemLibrary.K2_PauseTimerHandle` (`self.PatrolHandle`)))))

(fn `UserConstructionScript`)