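; BP_SimplePath is a path actor that defines a route with a PatrolSpline and lays spline meshes along it.
; Its construction script adds one SplineMeshComponent per segment between consecutive spline points, attached to DefaultSceneRoot.
; Each mesh takes its start and end positions and tangents from the spline in local space, so it follows the curve.
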(fn `UserConstructionScript`
  (bind _patrolspline (`self.PatrolSpline`))
  (for _index (range (+ (- (`SplineComponent.GetNumberOfSplinePoints` (`self.PatrolSpline`)) 2) 1))
    (bind _returnvalue (`AddComponent|NODE_AddSplineMeshComponent-0` :`bManualAttachment` true))
    (`SceneComponent.K2_AttachTo` _returnvalue (`self.DefaultSceneRoot`) "None" "KeepRelativeOffset" true)
    (bind (_location _tangent) (`SplineComponent.GetLocationAndTangentAtSplinePoint` _patrolspline _index "Local"))
    (bind (_location_2 _tangent_2) (`SplineComponent.GetLocationAndTangentAtSplinePoint` _patrolspline (+ _index 1) "Local"))
    (`SplineMeshComponent.SetStartAndEnd` _returnvalue _location _tangent _location_2 _tangent_2 true)))