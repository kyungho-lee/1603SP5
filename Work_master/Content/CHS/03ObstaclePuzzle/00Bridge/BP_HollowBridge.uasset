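; BP_HollowBridge is an obstacle-puzzle bridge with a gap that affects followers and responds to fill objects.
; When a JustFollow character overlaps StopFollowingDieOrSwim, its mesh starts simulating physics.
; When a BP_FillObject overlaps the same volume, ViewSize is set to block the Pawn channel.
; The StopActor overlap is empty, and leftover logic for pausing movement timers or destroying followers is disconnected.
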(event `self.StopActor.OnComponentBeginOverlap`
  (params (OverlappedComponent :type "PrimitiveComponent Object Reference") (OtherActor :type "Actor Object Reference") (OtherComp :type "PrimitiveComponent Object Reference") (OtherBodyIndex :type Integer) (bFromSweep :type Boolean) (SweepResult :type "HitResult Structure (by ref)")))

(event `self.StopFollowing(DieOrSwim).OnComponentBeginOverlap`
  (params (OverlappedComponent :type "PrimitiveComponent Object Reference") (OtherActor :type "Actor Object Reference") (OtherComp :type "PrimitiveComponent Object Reference") (OtherBodyIndex :type Integer) (bFromSweep :type Boolean) (SweepResult :type "HitResult Structure (by ref)"))
  (`|ExecutionSequence`
    (:`then_0`
      (bind _asjust_follow (cast `/Game/CHS/02FollowPathUnit/01SimplePathMover/JustFollow` OtherActor))
      (`PrimitiveComponent.SetSimulatePhysics` (`Character.Mesh` _asjust_follow) true))
    (:`then_1`
      (cast `/Game/CHS/03ObstaclePuzzle/02FillHole/BP_FillObject` OtherActor)
      (`PrimitiveComponent.SetCollisionResponseToChannel` (`self.ViewSize`) "ECC_Pawn" "ECR_Block"))))

(fn `UserConstructionScript`)