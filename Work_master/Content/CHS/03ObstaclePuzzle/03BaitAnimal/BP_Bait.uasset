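; BP_Bait is a throwable bait item for the bait-animal obstacle puzzle that can respawn after a throw.
; BeginPlay caches the Bait component's world location as the respawn point.
; Overlapping BP_BearFinal sets DestroyBool to the inverse of the bear's BaitBool.
; Throwed waits a fixed delay, then, if DestroyBool is set, spawns a fresh BP_Bait at the cached location and destroys itself.
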(event `self.ReceiveBeginPlay`
  (set `self.RespawnLoc` (`SceneComponent.K2_GetComponentLocation` (`self.Bait`))))

(event `CheckBait`
  (bind _asbp_bear_final (cast `/Game/CHS/03ObstaclePuzzle/03BaitAnimal/BP_BearFinal` (stale `self.Bait.OnComponentBeginOverlap` OtherActor) :!label _label))
  (if (`/Game/CHS/03ObstaclePuzzle/03BaitAnimal/BP_BearFinal.BaitBool` _asbp_bear_final)
    (set `self.DestroyBool` false)
    (else
      (set `self.DestroyBool` true))))

(event `self.Bait.OnComponentBeginOverlap`
  (params (OverlappedComponent :type "PrimitiveComponent Object Reference") (OtherActor :type "Actor Object Reference") (OtherComp :type "PrimitiveComponent Object Reference") (OtherBodyIndex :type Integer) (bFromSweep :type Boolean) (SweepResult :type "HitResult Structure (by ref)"))
  (goto _label))

(event `Throwed`
  (`KismetSystemLibrary.Delay` 4.0)
  (if (`self.DestroyBool`)
    (`|SpawnActorFromClass` "BP_Bait_C" (`KismetMathLibrary.MakeTransform` (`self.RespawnLoc`)) "Undefined" "OverrideRootScale" null null)
    (`/Engine/EditorBlueprintResources/StandardMacros.IsValid` self
      (:`Is Valid`
        (`self.K2_DestroyActor`)))))

(fn `UserConstructionScript`)