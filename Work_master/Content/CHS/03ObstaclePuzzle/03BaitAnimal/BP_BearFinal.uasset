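; BP_BearFinal is a bait target location in the bait-animal obstacle puzzle that notifies a bear when bait arrives.
; A bait overlapping the FinalLoc sphere starts a three-second timer.
; When it fires, a debug-drawn sphere trace at the actor, scaled up from FinalLoc's radius, looks for the bait again.
; A hit sets BaitBool and calls CheckBait on both the bait and the referenced Bear.
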(event `CheckStart`
  (`KismetSystemLibrary.K2_SetTimerDelegate` (delegate `BaitTickCheck`) 3.0))

(event `BaitTickCheck`
  (bind _returnvalue (`self.K2_GetActorLocation`))
  (bind (_outhit _returnvalue_2) (`KismetSystemLibrary.SphereTraceSingleForObjects` :`Start` _returnvalue :`End` _returnvalue :`Radius` (* 8 (`SphereComponent.SphereRadius` (`self.FinalLoc`))) :`ObjectTypes` (`|MakeArray` "ObjectTypeQuery10" :!type "EObjectTypeQuery Enum") :`DrawDebugType` "ForDuration"))
  (if _returnvalue_2
    (bind _asbp_bait (cast `/Game/CHS/03ObstaclePuzzle/03BaitAnimal/BP_Bait` (`.HitActor` (`GameplayStatics.BreakHitResult` _outhit))))
    (set `self.BaitBool` true)
    (`/Game/CHS/03ObstaclePuzzle/03BaitAnimal/BP_Bait.CheckBait` _asbp_bait)
    (`/Game/CHS/03ObstaclePuzzle/03BaitAnimal/BP_PolarBear.CheckBait` (`self.Bear`))))

(event `self.FinalLoc.OnComponentBeginOverlap`
  (params (OverlappedComponent :type "PrimitiveComponent Object Reference") (OtherActor :type "Actor Object Reference") (OtherComp :type "PrimitiveComponent Object Reference") (OtherBodyIndex :type Integer) (bFromSweep :type Boolean) (SweepResult :type "HitResult Structure (by ref)"))
  (cast `/Game/CHS/03ObstaclePuzzle/03BaitAnimal/BP_Bait` OtherActor)
  (`self.CheckStart`))

(fn `UserConstructionScript`)