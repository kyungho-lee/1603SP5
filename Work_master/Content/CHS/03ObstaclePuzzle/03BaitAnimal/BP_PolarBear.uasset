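; Polar bear character for the bait-animal obstacle puzzle that walks toward one of two goal actors.
; A looping timer started on BeginPlay repeatedly sets a fixed walk speed and issues a simple move-to through the bear's controller.
; It heads for FirstLoc until the CheckBait event sets ChangeGoal, after which the next timer tick redirects it to FinalLoc.
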(event `self.ReceiveBeginPlay`
  (bind _returnvalue (`KismetSystemLibrary.K2_SetTimerDelegate` (delegate `MoveToLocationEvent`) 0.2 true))
  (set `self.MoveHandler` _returnvalue))

(event `MoveToLocationEvent`
  (bind _returnvalue (`self.GetController` self))
  (set `CharacterMovementComponent.MaxWalkSpeed` 150.0 (`self.CharacterMovement`))
  (if (`self.ChangeGoal`)
    (`AIBlueprintHelperLibrary.SimpleMoveToActor` _returnvalue (`self.FinalLoc`))
    (else
      (`AIBlueprintHelperLibrary.SimpleMoveToActor` _returnvalue (`self.FirstLoc`)))))

(event `/Game/CHS/03ObstaclePuzzle/03BaitAnimal/BPI_CheckBait.CheckBait`
  (set `self.ChangeGoal` true))

(fn `UserConstructionScript`)