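; BP_PullActor is a spawner actor in a rope obstacle puzzle folder that creates physics-simulated TestSpawnActor instances.
; Its SpawnPullActor event spawns one at a random point in a small box around itself, then scales it up and enables collision and physics on its mesh.
; A looping timer for repeated spawning is left disconnected, so nothing in this Blueprint triggers the event.
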(event `self.ReceiveBeginPlay`)

(event `SpawnPullActor`
  (bind _returnvalue (`|SpawnActorFromClass` "/Game/CHS/03ObstaclePuzzle/01Rope/TestSpawnActor.TestSpawnActor_C" (`KismetMathLibrary.Conv_VectorToTransform` (`KismetMathLibrary.RandomPointInBoundingBox` (`self.K2_GetActorLocation`) (100.0 150.0 1.0))) "AdjustIfPossibleButAlwaysSpawn" "OverrideRootScale" null null))
  (`/Engine/EditorBlueprintResources/StandardMacros.IsValid` _returnvalue
    (:`Is Valid`
      (`self.SetActorRelativeScale3D` _returnvalue (2.0 6.0 2.0))
      (bind _staticmesh (`/Game/CHS/03ObstaclePuzzle/01Rope/TestSpawnActor.StaticMesh` _returnvalue))
      (`PrimitiveComponent.SetCollisionEnabled` _staticmesh "QueryAndPhysics")
      (`PrimitiveComponent.SetSimulatePhysics` _staticmesh true))))

(fn `UserConstructionScript`)