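; BP_EndGame is a stage goal trigger that shows the success screen once enough JustFollow actors enter its box.
; Each overlap sets ScoreCheck to the last index of all JustFollow actors, one below their count, and adds the arrival to a unique array.
; When that array's length equals ScoreCheck, it saves the length to BP_Instance as RemainFollow and calls ShowStageSuccess with Score as the maximum.
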(event `self.Box.OnComponentBeginOverlap`
  (params (OverlappedComponent :type "PrimitiveComponent Object Reference") (OtherActor :type "Actor Object Reference") (OtherComp :type "PrimitiveComponent Object Reference") (OtherBodyIndex :type Integer) (bFromSweep :type Boolean) (SweepResult :type "HitResult Structure (by ref)"))
  (bind _tempscore (`self.TempScore`))
  (bind _asjust_follow (cast `/Game/CHS/02FollowPathUnit/01SimplePathMover/JustFollow` OtherActor))
  (`|ExecutionSequence`
    (:`then_0`
      (bind _outactors (`GameplayStatics.GetAllActorsOfClass` "/Game/CHS/02FollowPathUnit/01SimplePathMover/JustFollow.JustFollow_C"))
      (for (_ _array_index) _outactors
        _)
      (set `self.ScoreCheck` _array_index))
    (:`then_1`
      (`KismetArrayLibrary.Array_AddUnique` (`self.FollowArray`) _asjust_follow)
      (set `self.TempScore` (`KismetArrayLibrary.Array_Length` (`self.FollowArray`)))
      (if (== (`self.TempScore`) (`self.ScoreCheck`))
        (bind _asbp_instance (cast `/Game/CHS/01BP/BP_Instance` (`GameplayStatics.GetGameInstance`)))
        (set `/Game/CHS/01BP/BP_Instance.RemainFollow` _tempscore _asbp_instance)
        (`/Game/sungwon/ingame/LibPlayUI.show stage success` (`self.Score`) _tempscore)))))

(fn `UserConstructionScript`)